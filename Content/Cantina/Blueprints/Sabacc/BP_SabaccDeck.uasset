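; Sabacc deck actor that builds, shuffles and deals physical cards, and forwards a dice-roll key to the Sabacc game mode.
; ResetDeck destroys existing cards and rebuilds a Vector2D array of suit and value: two zeros plus three signed suits.
; DealCard spawns a BP_SabaccCard, launches it toward a target and labels it.
; Its printout, removal and label use separate random picks, so they can refer to different cards.
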(event `self.ReceiveBeginPlay`
  (`|ExecutionSequence`
    (:`then_0`
      (bind _asbp_sabacc_game_mode (cast `/Game/Cantina/Blueprints/Sabacc/BP_SabaccGameMode` (`GameplayStatics.GetGameMode`)))
      (set `self.GM` _asbp_sabacc_game_mode))
    (:`then_1`
      (`self.ResetDeck`))))

(event `ResetDeck`
  (bind _deckarray (`self.DeckArray`))
  (bind _deckarray_2 (`self.DeckArray`))
  (bind _deckarray_3 (`self.DeckArray`))
  (bind _deckarray_4 (`self.DeckArray`))
  (bind _returnvalue (+ (`self.CurrentIteration`) 1))
  (bind _returnvalue_2 (+ (`self.CurrentIteration`) 1))
  (bind _returnvalue_3 (+ (`self.CurrentIteration`) 1))
  (`|ExecutionSequence`
    (:`then_0`
      ;[1 1 1] Reset everything
      (set `self.CurrentIteration` 0)
      (`KismetArrayLibrary.Array_Clear` (`self.DeckArray`))
      (set `self.DIscarded` 0)
      (set `self.DeckReady` false)
      (bind _outactors (`GameplayStatics.GetAllActorsOfClass` "/Game/Cantina/Blueprints/Sabacc/BP_SabaccCard.BP_SabaccCard_C"))
      (for _array_element _outactors
        (`self.K2_DestroyActor` _array_element)))
    (:`then_1`
      ;[1 1 1] Add zeros
      (`KismetArrayLibrary.Array_Add` _deckarray)
      (`KismetArrayLibrary.Array_Add` _deckarray))
    (:`then_2`
      ;[1 1 1] Generate circle suit
      (while (< (`self.CurrentIteration`) 10)
        (`KismetArrayLibrary.Array_Add` _deckarray_3 (`KismetMathLibrary.MakeVector2D` 1.0 (`KismetMathLibrary.Conv_IntToDouble` _returnvalue)))
        (`KismetArrayLibrary.Array_Add` _deckarray_3 (`KismetMathLibrary.MakeVector2D` 1.0 (`KismetMathLibrary.Conv_IntToDouble` (* _returnvalue -1))))
        (`/Engine/EditorBlueprintResources/StandardMacros.IncrementInt` (`self.CurrentIteration`)))
      (set `self.CurrentIteration` 0))
    (:`then_3`
      ;[1 1 1] Generate circle suit
      (while (< (`self.CurrentIteration`) 10)
        (`KismetArrayLibrary.Array_Add` _deckarray_4 (`KismetMathLibrary.MakeVector2D` 2.0 (`KismetMathLibrary.Conv_IntToDouble` _returnvalue_2)))
        (`KismetArrayLibrary.Array_Add` _deckarray_4 (`KismetMathLibrary.MakeVector2D` 2.0 (`KismetMathLibrary.Conv_IntToDouble` (* _returnvalue_2 -1))))
        (`/Engine/EditorBlueprintResources/StandardMacros.IncrementInt` (`self.CurrentIteration`)))
      (set `self.CurrentIteration` 0))
    (:`then_4`
      ;[1 1 1] Generate circle suit
      (while (< (`self.CurrentIteration`) 10)
        (`KismetArrayLibrary.Array_Add` _deckarray_2 (`KismetMathLibrary.MakeVector2D` 3.0 (`KismetMathLibrary.Conv_IntToDouble` _returnvalue_3)))
        (`KismetArrayLibrary.Array_Add` _deckarray_2 (`KismetMathLibrary.MakeVector2D` 3.0 (`KismetMathLibrary.Conv_IntToDouble` (* _returnvalue_3 -1))))
        (`/Engine/EditorBlueprintResources/StandardMacros.IncrementInt` (`self.CurrentIteration`)))
      (set `self.CurrentIteration` 0))
    (:`then_5`)
    (:`then_6`
      (`KismetArrayLibrary.Array_Shuffle` (`self.DeckArray`)))
    (:`then_7`
      (set `self.DeckReady` true))))

(event `ShuffleDeck`
  ;[1 1 1] Shuffle Deck
  (`KismetArrayLibrary.Array_Shuffle` (`self.DeckArray`)))

(event `Key|NumPadSix`
  (params (Key :type "Key Structure"))
  ;[1 1 1] Roll Dice
  (:`Pressed`
    (`/Game/Cantina/Blueprints/Sabacc/BP_SabaccGameMode.RollDice` (`self.GM`))))

(event `DealCard`
  (params (Target :type "Vector Structure"))
  (bind (_outitem _outindex) (`KismetArrayLibrary.Array_Random` (`self.DeckArray`)))
  (bind _returnvalue (`KismetTextLibrary.Conv_DoubleToText` (`.Y` (`KismetMathLibrary.BreakVector2D` _outitem)) "HalfToEven"))
  (bind _returnvalue_2 (cast `/Game/Cantina/Blueprints/Sabacc/E_Suits` (`KismetMathLibrary.Conv_Int64ToByte` (`KismetMathLibrary.Conv_DoubleToInt64` (`KismetMathLibrary.BreakVector2D` _outitem)))))
  (if (< (`self.DIscarded`) 62)
    (switch `/Game/Cantina/Blueprints/Sabacc/E_Suits` _returnvalue_2
      (:`NewEnumerator0`
        (`KismetSystemLibrary.PrintString` "Zero"))
      (:`NewEnumerator1`
        (`KismetSystemLibrary.PrintString` "Circle"))
      (:`NewEnumerator2`
        (`KismetSystemLibrary.PrintString` "Square"))
      (:`NewEnumerator3`
        (`KismetSystemLibrary.PrintString` "Triangle")))
    (`KismetSystemLibrary.PrintString` (`KismetStringLibrary.Conv_DoubleToString` (`.Y` (`KismetMathLibrary.BreakVector2D` _outitem))))
    (`KismetArrayLibrary.Array_Remove` (`self.DeckArray`) _outindex)
    (`/Engine/EditorBlueprintResources/StandardMacros.IncrementInt` (`self.DIscarded`)
      (:`  `
        (bind _returnvalue_3 (`|SpawnActorFromClass` "/Game/Cantina/Blueprints/Sabacc/BP_SabaccCard.BP_SabaccCard_C" (`self.GetTransform`) "AlwaysSpawn" "MultiplyWithRoot" null null))
        (`PrimitiveComponent.SetPhysicsLinearVelocity` (`/Game/Cantina/Blueprints/Sabacc/BP_SabaccCard.StaticMesh` _returnvalue_3) (* (`KismetMathLibrary.GetDirectionUnitVector` (`self.K2_GetActorLocation` _returnvalue_3) Target) (130.0 130.0 -10.0)) false "None")
        (switch `/Game/Cantina/Blueprints/Sabacc/E_Suits` (cast `/Game/Cantina/Blueprints/Sabacc/E_Suits` _returnvalue_2)
          (:`NewEnumerator0`
            (`/Game/Cantina/Blueprints/Sabacc/BP_SabaccCard.SetText` _returnvalue_3 (`|FormatText` "0")))
          (:`NewEnumerator1`
            (`/Game/Cantina/Blueprints/Sabacc/BP_SabaccCard.SetText` _returnvalue_3 (`|FormatText` "C{n}" _returnvalue)))
          (:`NewEnumerator2`
            (`/Game/Cantina/Blueprints/Sabacc/BP_SabaccCard.SetText` _returnvalue_3 (`|FormatText` "S{n}" _returnvalue)))
          (:`NewEnumerator3`
            (`/Game/Cantina/Blueprints/Sabacc/BP_SabaccCard.SetText` _returnvalue_3 (`|FormatText` "T{n}" _returnvalue))))))))

(fn `UserConstructionScript`)