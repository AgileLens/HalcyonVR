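; Game mode for a Sabacc card game that resets the deck and deals five rounds to four player zones.
; BeginPlay finds the deck actor and maps BP_DealZone locations to seats by player number.
; Looping timers drive DealRound and DealCard, with DoN counters cycling seats through the deck's DealCard and debug prints.
; RollDice randomizes and prints a gold value and suit but is not called here; ResetGame is an empty stub.
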(event `ResetGame`)

(event `self.ReceiveBeginPlay`
  (`|ExecutionSequence`
    (:`then_0`
      (`KismetArrayLibrary.Array_Clear` (`self.DealZones`)))
    (:`then_1`
      (bind _returnvalue (`GameplayStatics.GetActorOfClass` "/Game/Cantina/Blueprints/Sabacc/BP_SabaccDeck.BP_SabaccDeck_C"))
      (set `self.SabaccDeckRef` _returnvalue))
    (:`then_2`
      (bind _outactors (`GameplayStatics.GetAllActorsOfClass` "/Game/Cantina/Blueprints/Sabacc/BP_DealZone.BP_DealZone_C"))
      (for _array_element _outactors
        (switch `int` (`/Game/Cantina/Blueprints/Sabacc/BP_DealZone.PlayerNumber` _array_element)
          (:`0`
            (bind _returnvalue_2 (`self.K2_GetActorLocation` _array_element))
            (set `self.Player1Zone` _returnvalue_2))
          (:`1`
            (set `self.Player2Zone` _returnvalue_2))
          (:`2`
            (set `self.Player3Zone` _returnvalue_2))
          (:`3`
            (set `self.Player4Zone` _returnvalue_2)))))
    (:`then_3`
      (set `self.PlayerZones` (`|MakeArray` (`self.Player1Zone`) (`self.Player2Zone`) (`self.Player3Zone`) (`self.Player4Zone`))))
    (:`then_4`
      (`|ExecutionSequence`
        (:`then_0`
          (`KismetSystemLibrary.PrintString` "STARTING DEALING ROUND"))
        (:`then_1`
          (`/Game/Cantina/Blueprints/Sabacc/BP_SabaccDeck.ResetDeck` (`self.SabaccDeckRef`)))
        (:`then_2`
          (`KismetSystemLibrary.K2_SetTimerDelegate` (delegate `DealRound`) 1.0 true))))))

(event `RollDice`
  (bind _output_get (set `self.CurrentGold` (`KismetArrayLibrary.Array_Random` (`self.GoldDieValues`))))
  (bind _output_get_2 (set `self.CurrentSuit` (`KismetMathLibrary.RandomIntegerInRange` 1 3)))
  (`KismetSystemLibrary.PrintText` (`|FormatText` "Suit: {s} \nNum: {n}" _output_get_2 _output_get)))

(event `DealRound`
  (`/Engine/EditorBlueprintResources/StandardMacros.Do N` 5
    (:`Exit`
      (`KismetSystemLibrary.K2_SetTimerDelegate` (delegate `DealCard`) 0.4 true))))

(event `DealCard`
  (if (< (`self.RoundsDealt`) 5)
    (bind _counter (`/Engine/EditorBlueprintResources/StandardMacros.Do N` 4 :!label _label)
      (:`Exit`
        (bind _output (`|GetArrayItem` (`KismetStringLibrary.ParseIntoArray` "0,1,2,3" ",") (- _counter 1)))
        (`KismetSystemLibrary.PrintString` _output)
        (bind _output_2 (`|GetArrayItem` (`self.PlayerZones`) (`KismetStringLibrary.Conv_StringToInt` _output)))
        (`KismetSystemLibrary.PrintString` (`KismetStringLibrary.Conv_VectorToString` _output_2))
        (`/Game/Cantina/Blueprints/Sabacc/BP_SabaccDeck.DealCard` (`self.SabaccDeckRef`) _output_2)
        (if (== _counter 4)
          (`/Engine/EditorBlueprintResources/StandardMacros.IncrementInt` (`self.RoundsDealt`)
            (:`  `
              (goto _label :!via `Reset`))))))))

(fn `UserConstructionScript`)