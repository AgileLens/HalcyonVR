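; Blueprint library helper that plays a haptic tick on both of the first player's controllers as a tracked value reaches multiples of an increment.
; Rotation values are normalized and offset to a positive range before a modulo test, using a tolerance derived from the increment.
; A DoOnce prevents repeat pulses, re-arming only when the remainder lands in the narrow band just beyond the trigger window.
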(fn `HapticOnChange`
  (params (Haptic :type "HapticFeedbackEffect_Base Object Reference") (FloatToTrack :type "Float (double-precision)" :default 0.0) (Increment :type "Float (double-precision)" :default 1.0) (`bIsRotation?` :type Boolean))
  (locals (HapticEffect :type "HapticFeedbackEffect_Base Object Reference" :default "/Script/Engine.HapticFeedbackEffect_Curve'/Game/VRTemplate/Haptics/GrabHapticEffect.GrabHapticEffect'") (Value :type "Float (double-precision)") (Buffer :type "Float (double-precision)" :default 5.0))
  (bind _returnvalue (`GameplayStatics.GetPlayerController` null))
  (bind _hapticeffect (`local.HapticEffect`))
  (bind _buffer (`local.Buffer`))
  (bind _returnvalue_2 (mod (`local.Value`) Increment))
  (set `local.Buffer` (/ Increment 7.0))
  (set `local.HapticEffect` Haptic)
  (if `bIsRotation?`
    (set `local.Value` (+ (`KismetMathLibrary.NormalizeAxis` FloatToTrack) 180.0))
    (else
      (set `local.Value` FloatToTrack)))
  (if (`KismetMathLibrary.NearlyEqual_FloatFloat` _returnvalue_2 0.0 _buffer)
    (`/Engine/EditorBlueprintResources/StandardMacros.DoOnce` false :!label _label
      (:`Completed`
        (`PlayerController.PlayHapticEffect` _returnvalue _hapticeffect "Left" 1.0 false)
        (`PlayerController.PlayHapticEffect` _returnvalue _hapticeffect "Right" 1.0 false)))
    (elif (`KismetMathLibrary.NearlyEqual_FloatFloat` _returnvalue_2 _buffer _buffer)
      (goto _label :!via `Reset`))))