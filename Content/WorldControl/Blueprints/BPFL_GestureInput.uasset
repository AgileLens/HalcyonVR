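; Blueprint function library that detects XR hand-tracking gestures and draws tracked hands with instanced static meshes.
; SetupHands adds instances to both hands' finger meshes.
; HandBonesTouchCheck moves those instances to each keypoint, scaled by radius, then returns a touch state from two keypoints' distance against a threshold, plus the first point's location.
; PalmDownCheck tests keypoint 0's raw quaternion X and Y against per-hand ranges.
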(fn `HandBonesTouchCheck`
  (params (Hand :type "EControllerHand Enum" :default "Left") (BonePointA :type "EHandKeypoint Enum" :default "Palm") (BonePointB :type "EHandKeypoint Enum" :default "Palm") (ISM_Fingers :type "InstancedStaticMeshComponent Object Reference") (DistThreshold :type "Float (double-precision)"))
  (returns (InputState :type "/Game/WorldControl/Blueprints/EInputState Enum") (PointA_Loc :type "Vector Structure (by ref)"))
  (locals (bGestureIsActive :type Boolean) (`Local BonePointA` :type "EHandKeypoint Enum") (`Local BonePointB` :type "EHandKeypoint Enum") (MotionControllerData :type "XRMotionControllerData Structure") (`Local Hand` :type "EControllerHand Enum") (`Local ISM_Fingers` :type "InstancedStaticMeshComponent Object Reference") (`Local DistThreshold` :type "Float (double-precision)"))
  (bind (_bvalid _devicename _applicationinstanceid _devicevisualtype _handindex _trackingstatus _gripposition _griprotation _aimposition _aimrotation _palmposition _palmrotation _handkeypositions _handkeyrotations _handkeyradii) (break `XRMotionControllerData` (`local.MotionControllerData`)))
  (bind _output (`|GetArrayItem` _handkeypositions (`HandKeypointConversion.Conv_HandKeypointToInt32` (`local.Local BonePointA`))))
  (set `local.Local Hand` Hand)
  (set `local.Local BonePointA` BonePointA)
  (set `local.Local BonePointB` BonePointB)
  (set `local.Local ISM_Fingers` ISM_Fingers)
  (set `local.Local DistThreshold` DistThreshold)
  ;[1 1 1] Update Finger Data
  (bind _motioncontrollerdata (`HeadMountedDisplayFunctionLibrary.GetMotionControllerData` null (`local.Local Hand`)))
  (set `local.MotionControllerData` _motioncontrollerdata)
  (if _bvalid
    (`|ExecutionSequence`
      (:`then_0`
        (bind _enumvalue (foreach `EHandKeypoint` false)
          (:`LoopBody`
            (bind _output_2 (`|GetArrayItem` _handkeyradii (`HandKeypointConversion.Conv_HandKeypointToInt32` _enumvalue)))
            (bind _returnvalue (* _output_2 0.01))
            (`InstancedStaticMeshComponent.UpdateInstanceTransform` (`local.Local ISM_Fingers`) 0 (`KismetMathLibrary.MakeTransform` (`|GetArrayItem` _handkeypositions (`HandKeypointConversion.Conv_HandKeypointToInt32` _enumvalue)) (`KismetMathLibrary.Quat_Rotator` (`|GetArrayItem` _handkeyrotations (`HandKeypointConversion.Conv_HandKeypointToInt32` _enumvalue))) (`KismetMathLibrary.MakeVector` _returnvalue (* _output_2 0.036) _returnvalue)) true true true))))
      (:`then_1`
        ;[1 1 1] Have the fingers started touching or stopped touching?
        (bind _output_get (set `local.bGestureIsActive` (< (`KismetMathLibrary.Vector_Distance` _output (`|GetArrayItem` _handkeypositions (`HandKeypointConversion.Conv_HandKeypointToInt32` (`local.Local BonePointB`)))) (`local.Local DistThreshold`))))
        (if _output_get
          (return "NewEnumerator2" _output)
          (else
            (return "NewEnumerator3" _output)))))
    (else
      (return "NewEnumerator0" (0.0 0.0 0.0)))))

(fn `PalmDownCheck`
  (params (Hand :type "EControllerHand Enum" :default "Left"))
  (returns (InputState :type "/Game/WorldControl/Blueprints/EInputState Enum"))
  (locals (bGestureIsActive :type Boolean) (`Local BonePointA` :type "EHandKeypoint Enum") (`Local BonePointB` :type "EHandKeypoint Enum") (MotionControllerData :type "XRMotionControllerData Structure") (`Local Hand` :type "EControllerHand Enum") (`Local ISM_Fingers` :type "InstancedStaticMeshComponent Object Reference") (`Local DistThreshold` :type "Float (double-precision)"))
  (bind _output_get (set `local.Local Hand` Hand))
  ;[1 1 1] Update Finger Data
  (bind _motioncontrollerdata (`HeadMountedDisplayFunctionLibrary.GetMotionControllerData` null _output_get))
  (bind _output_get_2 (set `local.MotionControllerData` _motioncontrollerdata))
  (bind (_bvalid _devicename _applicationinstanceid _devicevisualtype _handindex _trackingstatus _gripposition _griprotation _aimposition _aimrotation _palmposition _palmrotation _handkeypositions _handkeyrotations) (break `XRMotionControllerData` _output_get_2))
  (if _bvalid
    (bind (_x _y) (`KismetMathLibrary.BreakQuat` (`|GetArrayItem` _handkeyrotations)))
    (bind _output_get_3 (set `local.bGestureIsActive` (or (and (and (> _x 0.1) (< _x 0.7)) (and (> _y -0.1) (< _y 0.5)) (`|EnumEquality` (`local.Local Hand`) "Left")) (and (and (> _x 0.1) (< _x 0.7)) (and (> _y -0.4) (< _y 0.1)) (`|EnumEquality` (`local.Local Hand`) "Right")))))
    (if _output_get_3
      (return "NewEnumerator1")
      (else
        (return "NewEnumerator0")))
    (else
      (return "NewEnumerator0"))))

(fn `SetupHands`
  (params (ISM_Fingers_Left :type "InstancedStaticMeshComponent Object Reference") (ISM_Fingers_Right :type "InstancedStaticMeshComponent Object Reference"))
  (locals (`Local ISM_Fingers_Right` :type "InstancedStaticMeshComponent Object Reference") (`Local ISM_Fingers_Left` :type "InstancedStaticMeshComponent Object Reference"))
  (bind _returnvalue (`KismetMathLibrary.MakeTransform` (0.0 0.0 0.0)))
  (set `local.Local ISM_Fingers_Left` ISM_Fingers_Left)
  (set `local.Local ISM_Fingers_Right` ISM_Fingers_Right)
  (foreach `EHandKeypoint` false
    (:`LoopBody`
      (`InstancedStaticMeshComponent.AddInstance` ISM_Fingers_Left _returnvalue false)
      (`InstancedStaticMeshComponent.AddInstance` ISM_Fingers_Right _returnvalue false)
      (return))))