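; BP_Picture is a VR picture actor with a configurable texture that can be stuck onto a surface while held.
; UpdateTexture applies TextureParam through a dynamic material instance, both at construction and at BeginPlay.
; TriggerPressed traces along the actor's negative up vector, detaches it and teleports it to the hit, aligned to the surface normal with a slight offset.
; It then plays a haptic on the hand read from GrabComponent.
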(event `self.ReceiveBeginPlay`
  (`self.UpdateTexture`))

(event `UpdateTexture`
  (bind _staticmesh (`self.StaticMesh`))
  (bind _returnvalue (`PrimitiveComponent.CreateDynamicMaterialInstance` _staticmesh 0 (`PrimitiveComponent.GetMaterial` _staticmesh 0) "Texture_"))
  (`MaterialInstanceDynamic.SetTextureParameterValue` _returnvalue "Texture" (`self.TextureParam`))
  (`PrimitiveComponent.SetMaterial` _staticmesh 0 _returnvalue))

(event `/Game/VRTemplate/Blueprints/VRInteractionBPI.TriggerPressed`
  (bind _returnvalue (`self.K2_GetActorLocation`))
  (bind _outhit (`KismetSystemLibrary.LineTraceSingleForObjects` :`Start` _returnvalue :`End` (+ _returnvalue (* (`self.GetActorUpVector`) -500.0)) :`ObjectTypes` (`self.Object Types`) :`bIgnoreSelf` false))
  (`self.K2_DetachFromActor` "KeepWorld" "KeepWorld" "KeepWorld")
  (`self.K2_SetActorLocationAndRotation` (`.Location` (`GameplayStatics.BreakHitResult` _outhit)) (`KismetMathLibrary.Conv_VectorToRotator` (`.ImpactNormal` (`GameplayStatics.BreakHitResult` _outhit))) false true)
  (`self.K2_AddActorLocalRotation` (struct :`Yaw` -90.0 :`Roll` 90.0) false true)
  (`self.K2_AddActorLocalOffset` (0.0 0.0 1.0) false true)
  (`PlayerController.PlayHapticEffect` (`GameplayStatics.GetPlayerController` 0) "/Game/VRTemplate/Haptics/PistolFireHapticEffect.PistolFireHapticEffect" (select `bool` (== (`MotionControllerComponent.MotionSource` (`/Game/VRTemplate/Blueprints/GrabComponent.MotionControllerRef` (`self.GrabComponent`))) "Left") :`false` "Right" :`true` "Left" :!type "EControllerHand Enum") 1.0 false))

(fn `UserConstructionScript`
  (`self.UpdateTexture`))