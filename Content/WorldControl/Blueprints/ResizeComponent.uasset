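; Actor component that lets its owning actor be resized with two hands, adding a Grab Component at BeginPlay if the owner lacks one.
; BeginResize stores both hands, their starting distance and the actor's initial scale, then turns on tick.
; Tick scales the actor by the ratio of current to initial hand distance and passes that ratio to HapticOnChange for incremental haptic feedback.
; EndResize turns tick back off.
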(event `self.ReceiveBeginPlay`
  ;[0 0.6449 1] If Actor doesn't also have Grab Component, add it
  (bind _output_get (set `self.OwningActor` (`self.GetOwner`)))
  (`/Engine/EditorBlueprintResources/StandardMacros.IsValid` (`Actor.GetComponentByClass` _output_get "/Game/VRTemplate/Blueprints/GrabComponent.GrabComponent_C")
    (:`Is Not Valid`
      (`|AddComponentByClass` :`self` (`self.OwningActor`) :`Class` "/Game/VRTemplate/Blueprints/GrabComponent.GrabComponent_C"))))

(event `/Game/WorldControl/Blueprints/ResizeActorInterface.BeginResize`
  (params (FirstHand :type "SceneComponent Object Reference") (SecondHand :type "SceneComponent Object Reference"))
  (`self.SetComponentTickEnabled` true)
  (set `self.FirstHand` FirstHand)
  (set `self.SecondHand` SecondHand)
  (set `self.bIsResizing` true)
  (bind _distance (`/Game/WorldControl/Blueprints/BPFL_GetDistance.GetDistance` (`self.FirstHand`) (`self.SecondHand`)))
  (set `self.InitialDistance` _distance)
  (bind _output_get (set `self.InitialScale` (`Actor.GetActorScale3D` (`self.GetOwner`))))
  (`KismetSystemLibrary.PrintString` (`KismetStringLibrary.Concat_StrStr` "Initial Scale: " (`KismetStringLibrary.Conv_VectorToString` _output_get))))

(event `self.ReceiveTick`
  (params (DeltaSeconds :type "Float (single-precision)"))
  (if (`self.bIsResizing`)
    (bind _distance (`/Game/WorldControl/Blueprints/BPFL_GetDistance.GetDistance` (`self.FirstHand`) (`self.SecondHand`)))
    (bind _returnvalue (/ _distance (`self.InitialDistance`)))
    (bind _output_get (set `self.CurrentScale` (* (`self.InitialScale`) _returnvalue)))
    (`Actor.SetActorScale3D` (`self.GetOwner`) _output_get)
    (`/Game/WorldControl/Blueprints/BPFL_HapticOnChange.HapticOnChange` "/Game/WorldControl/Haptics/ResizingHapticEffect.ResizingHapticEffect" _returnvalue 0.2)))

(event `/Game/WorldControl/Blueprints/ResizeActorInterface.EndResize`
  (set `self.bIsResizing` false)
  (`self.SetComponentTickEnabled` false)
  (`KismetSystemLibrary.PrintString` (`KismetStringLibrary.Concat_StrStr` "End Scale: " (`KismetStringLibrary.Conv_VectorToString` (`self.CurrentScale`)))))