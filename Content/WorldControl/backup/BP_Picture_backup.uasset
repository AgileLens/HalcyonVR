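; Backup of a VR picture actor, apparently meant to snap from the hand onto a surface, though no event triggers its only logic.
; The unwired chain releases the VRPawn grab for the hand in GrabComponent, waits briefly, then detaches the actor.
; It moves the picture to a line trace hit along its negative up axis, aligns it to the surface normal and plays haptics on that hand.
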(fn `UserConstructionScript`)