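; Collaborative Viewer command component for the "3D Cut Volume" tool, with Add/Edit, Remove and Include/Exclude option buttons.
; Button bindings spawn a single BP_CropBox at the hand laser's hit point, destroy it, or flip its include/exclude state.
; Add/Edit uses a macro that polls until the box is valid on the client, then shows its gizmo and switches pawn collision types, which are reset on disable.
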(event `self.ReceiveBeginPlay`
  ;[0 1 0.1488] Begin Play
  (set `self.Icon` "/Game/CollaborativeViewer/Blueprints/Commands/CropBox/3D_Cut_Icon.3D_Cut_Icon")
  (`|ExecutionSequence`
    (:`then_0`
      (bind _outactors (`GameplayStatics.GetAllActorsOfClass` "/Game/CollaborativeViewer/Blueprints/Commands/CropBox/BPs/BP_CropBox.BP_CropBox_C"))
      (if (> (`KismetArrayLibrary.Array_Length` _outactors) 0)
        (`/Game/CollaborativeViewer/Blueprints/Commands/CropBox/BPs/BP_CropBox.ShowGizmo` (`|GetArrayItem` _outactors) false)))))

(event `self.ExecuteAfterSpawnPawn`
  ;[0 1 0.1488] Begin Play
  (`parent.ExecuteAfterSpawnPawn`)
  (`|ExecutionSequence`
    (:`then_0`
      (set `self.OptionsButtonNames` (`|MakeArray` "ADD / EDIT" "REMOVE" "INCLUDE / EXCLUDE" :!type "Text"))
      (set `self.Name` "3D Cut Volume"))
    (:`then_1`
      (`self.CreateContextualButon`)
      (`self.BindADDEdit`)
      (`self.BindRemoveButton`)
      (`self.BindExcludeInclude`))))

(event `TransformUpdateOnServer`
  (params (Transform :type "Transform Structure") (cutplane :type "/Game/CollaborativeViewer/Blueprints/Commands/CropBox/BPs/BP_CropBox Object Reference"))
  ;[0.2555 0.7775 1] Update Transform on Server
  (`/Engine/EditorBlueprintResources/StandardMacros.IsValid` cutplane
    (:`Is Valid`
      (set `/Game/CollaborativeViewer/Blueprints/Commands/CropBox/BPs/BP_CropBox.TransformUpdate` Transform cutplane))))

(event `Create3DcutCube`
  (params (Pawn :type "/Game/CollaborativeViewer/Blueprints/Pawn/BP_BasePawn Object Reference") (ISRight :type Boolean))
  ;[0.2555 0.7775 1] Create / Destroy Cut Cube
  (bind _outactors (`GameplayStatics.GetAllActorsOfClass` "/Game/CollaborativeViewer/Blueprints/Commands/CropBox/BPs/BP_CropBox.BP_CropBox_C"))
  (`/Engine/EditorBlueprintResources/StandardMacros.IsValid` (`|GetArrayItem` _outactors)
    (:`Is Not Valid`
      (`|SpawnActorFromClass` "/Game/CollaborativeViewer/Blueprints/Commands/CropBox/BPs/BP_CropBox.BP_CropBox_C" (`KismetMathLibrary.MakeTransform` (`/Game/CollaborativeViewer/Blueprints/Pawn/Laser.HitLaserEnd` (select `bool` ISRight :`false` (`/Game/CollaborativeViewer/Blueprints/Pawn/BP_BasePawn.LaserActor_L` Pawn) :`true` (`/Game/CollaborativeViewer/Blueprints/Pawn/BP_BasePawn.LaserActor_r` Pawn)))) "Undefined" "OverrideRootScale" null null null))))

(event `DestroyCutCubeOnserver`
  ;[0.2555 0.7775 1] Create / Destroy Cut Cube
  (bind _outactors (`GameplayStatics.GetAllActorsOfClass` "/Game/CollaborativeViewer/Blueprints/Commands/CropBox/BPs/BP_CropBox.BP_CropBox_C"))
  (bind _output (`|GetArrayItem` _outactors))
  (`/Engine/EditorBlueprintResources/StandardMacros.IsValid` _output
    (:`Is Valid`
      (`Actor.K2_DestroyActor` _output))))

(event `BindRemoveButton`
  (bind _asoption_button (cast `/Game/CollaborativeViewer/UMG/GameMenu/Option_Button` (`|GetArrayItem` (`self.OptionsButtons`) 1) :!pure true))
  ;[0.2555 0.7775 1] Bind Options
  (set `/Game/CollaborativeViewer/UMG/GameMenu/Option_Button.WhenExecute` "NewEnumerator1" _asoption_button)
  (add `/Game/CollaborativeViewer/UMG/GameMenu/Option_Button.Execute` _asoption_button (delegate `DestroyCutPlane`)))

(event `DestroyCutPlane`
  (params (id :type Integer) (Actor :type "Actor Object Reference") (IsRightHand :type Boolean))
  ;[0.2555 0.7775 1] Bind Options
  (`self.DestroyCutCubeOnserver`))

(event `BindADDEdit`
  (bind _asoption_button (cast `/Game/CollaborativeViewer/UMG/GameMenu/Option_Button` (`|GetArrayItem` (`self.OptionsButtons`)) :!pure true))
  ;[0.2555 0.7775 1] Bind Options
  (set `/Game/CollaborativeViewer/UMG/GameMenu/Option_Button.WhenExecute` "NewEnumerator0" _asoption_button)
  (add `/Game/CollaborativeViewer/UMG/GameMenu/Option_Button.Execute` _asoption_button (delegate `CustomEvent_1`))
  (add `/Game/CollaborativeViewer/UMG/GameMenu/Option_Button.ExecuteMenuOn` _asoption_button (delegate `CustomEvent_2`))
  (add `/Game/CollaborativeViewer/UMG/GameMenu/Option_Button.Disabled` _asoption_button (delegate `OnCommandDisabled`)))

(event `OnCommandDisabled`
  ;[0.2555 0.7775 1] Bind Options
  (bind _3dcutplane (`self.FireWhenCutPlaneValidOnClient` false)
    (:`Is Valid`
      (`/Game/CollaborativeViewer/Blueprints/Commands/CropBox/BPs/BP_CropBox.ShowGizmo` _3dcutplane false)
      (set `/Game/CollaborativeViewer/Blueprints/Pawn/BP_BasePawn.CollisionType` (`|MakeArray` "ObjectTypeQuery2" "ObjectTypeQuery1" :!type "EObjectTypeQuery Enum") (`self.BasePawn`)))))

(event `CustomEvent_1`
  (params (id :type Integer) (Actor :type "Actor Object Reference") (IsRightHand :type Boolean))
  ;[0.2555 0.7775 1] Bind Options
  (`self.Create3DcutCube` (`self.BasePawn`) IsRightHand)
  (bind _3dcutplane (`self.FireWhenCutPlaneValidOnClient` false :!label _label)
    (:`Is Valid`
      (`/Game/CollaborativeViewer/Blueprints/Commands/CropBox/BPs/BP_CropBox.ShowGizmo` _3dcutplane true)
      (`/Game/CollaborativeViewer/Blueprints/Commands/CropBox/BPs/BP_CropBox.StartAnim` _3dcutplane)
      (set `/Game/CollaborativeViewer/Blueprints/Pawn/BP_BasePawn.CollisionType` (`|MakeArray` "ObjectTypeQuery11" :!type "EObjectTypeQuery Enum") (`self.BasePawn`)))))

(event `CustomEvent_2`
  ;[0.2555 0.7775 1] Bind Options
  (goto _label))

(event `BindExcludeInclude`
  (bind _asoption_button (cast `/Game/CollaborativeViewer/UMG/GameMenu/Option_Button` (`|GetArrayItem` (`self.OptionsButtons`) 2) :!pure true))
  ;[0.2555 0.7775 1] Bind Options
  (set `/Game/CollaborativeViewer/UMG/GameMenu/Option_Button.WhenExecute` "NewEnumerator1" _asoption_button)
  (add `/Game/CollaborativeViewer/UMG/GameMenu/Option_Button.Execute` _asoption_button (delegate `Flip`)))

(event `Flip`
  (params (id :type Integer) (Actor :type "Actor Object Reference") (IsRightHand :type Boolean))
  ;[0.2555 0.7775 1] Bind Options
  (`self.IncludeROS`))

(event `IncludeROS`
  ;[0.2555 0.7775 1] Bind Options
  (bind _outactors (`GameplayStatics.GetAllActorsOfClass` "/Game/CollaborativeViewer/Blueprints/Commands/CropBox/BPs/BP_CropBox.BP_CropBox_C"))
  (bind _output (`|GetArrayItem` _outactors))
  (`/Engine/EditorBlueprintResources/StandardMacros.IsValid` _output
    (:`Is Valid`
      (`/Game/CollaborativeViewer/Blueprints/Commands/CropBox/BPs/BP_CropBox.SetExcludeInclude` _output))))