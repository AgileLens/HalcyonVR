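; Collaborative Viewer Xray command component with Apply, Isolate and Reset all options for making actors see-through.
; Server/multicast event pairs resolve actors by CollabName tags, swap mesh materials and collision type, and tag them Locked_XRAY.
; Isolate x-rays the rest of the picked actor's attachment hierarchy.
; A spawned XrayManager stores affected actors and original materials for reset, which also updates the crop box, and for save/load.
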(event `self.BeginPLayEditor`
  ;[0 1 0.1488] BeginPLay
  (`self.CreateXrayManager` :!label _label))

(event `CreateXrayManager`
  ;[0.2555 0.7775 1] Create Manager On server
  (bind _returnvalue (`GameplayStatics.GetActorOfClass` "/Game/CollaborativeViewer/Blueprints/Commands/Xray/BPs/XrayManager.XrayManager_C"))
  (`/Engine/EditorBlueprintResources/StandardMacros.IsValid` _returnvalue
    (:`Is Valid`
      (set `self.XrayManager` _returnvalue))
    (:`Is Not Valid`
      (bind _returnvalue_2 (`|SpawnActorFromClass` "/Game/CollaborativeViewer/Blueprints/Commands/Xray/BPs/XrayManager.XrayManager_C" (`KismetMathLibrary.MakeTransform` (0.0 0.0 0.0)) "Undefined" "OverrideRootScale" null null))
      (set `self.XrayManager` _returnvalue_2))))

(event `self.ReceiveBeginPlay`
  ;[0 1 0.1488] BeginPLay
  (if (`KismetSystemLibrary.IsStandalone`)
    (goto _label)
    (else
      (bind _aspawn (cast `Pawn` (`self.GetOwner`)))
      ;;[1 1 1] Controlled Yet ?  Then
      (if (`Pawn.IsPlayerControlled` _aspawn) :!label _label_2
        (if (`Pawn.IsLocallyControlled` _aspawn)
          (goto _label))
        (else
          (`KismetSystemLibrary.Delay` 0.2)
          (goto _label_2))))))

(event `self.DestroyInEditor`
  ;[0.2555 0.7775 1] On DEstroy
  (`Actor.K2_DestroyActor` (`self.XrayManager`)))

(event `self.ExecuteAfterSpawnPawn`
  ;[0 1 0.1488] BeginPLay
  (`parent.ExecuteAfterSpawnPawn`)
  (set `self.Icon` "/Game/CollaborativeViewer/Blueprints/Commands/Xray/IconXray.IconXray")
  (set `self.OptionsButtonNames` (`|MakeArray` "Apply" "Isolate" "Reset all" :!type "Text"))
  (set `self.Name` "Xray")
  (`self.CreateContextualButon`)
  (`self.Bind_Options`)
  (`self.BindSaveGame` (`self.Persistent UI`)))

(event `Bind_Options`
  (bind _asoption_button (cast `/Game/CollaborativeViewer/UMG/GameMenu/Option_Button` (`|GetArrayItem` (`self.OptionsButtons`) 1) :!pure true))
  (bind _asoption_button_2 (cast `/Game/CollaborativeViewer/UMG/GameMenu/Option_Button` (`|GetArrayItem` (`self.OptionsButtons`)) :!pure true))
  (bind _asoption_button_3 (cast `/Game/CollaborativeViewer/UMG/GameMenu/Option_Button` (`|GetArrayItem` (`self.OptionsButtons`) 2) :!pure true))
  ;[0.2555 0.7775 1] Setup Option Buttons
  (`|ExecutionSequence`
    (:`then_0`
      (set `/Game/CollaborativeViewer/UMG/GameMenu/Option_Button.WhenExecute` "NewEnumerator0" _asoption_button_2)
      (add `/Game/CollaborativeViewer/UMG/GameMenu/Option_Button.Execute` _asoption_button_2 (delegate `Option1`)))
    (:`then_1`
      (set `/Game/CollaborativeViewer/UMG/GameMenu/Option_Button.WhenExecute` "NewEnumerator0" _asoption_button)
      (add `/Game/CollaborativeViewer/UMG/GameMenu/Option_Button.Execute` _asoption_button (delegate `Option2`)))
    (:`then_2`
      (set `/Game/CollaborativeViewer/UMG/GameMenu/Option_Button.WhenExecute` "NewEnumerator1" _asoption_button_3)
      (add `/Game/CollaborativeViewer/UMG/GameMenu/Option_Button.Execute` _asoption_button_3 (delegate `Option3`)))))

(event `Option1`
  (params (id :type Integer) (Actor :type "Actor Object Reference") (IsRightHand :type Boolean))
  (bind (_actorname _tag_found) (`/Game/CollaborativeViewer/Blueprints/ShareLibrary/CommonFunctions_CV.GetCollabTag` Actor))
  ;[0.2555 0.7775 1] Setup Option Buttons
  (bind _locked (`/Game/CollaborativeViewer/Blueprints/ShareLibrary/CommonFunctions_CV.Is Actor Locked With Tag` Actor))
  (if _locked
    _
    (elif _tag_found
      (`self.ApplyXray_ROS` _actorname))))

(event `Option2`
  (params (id :type Integer) (Actor :type "Actor Object Reference") (IsRightHand :type Boolean))
  ;[0.2555 0.7775 1] Setup Option Buttons
  (bind _locked (`/Game/CollaborativeViewer/Blueprints/ShareLibrary/CommonFunctions_CV.Is Actor Locked With Tag` Actor))
  (if (not _locked)
    (`self.SetIsolateArrayActors` Actor)
    (`self.IsolateXrayROS` (`self.IsolatedActorArray`))))

(event `Option3`
  (params (id :type Integer) (Actor :type "Actor Object Reference") (IsRightHand :type Boolean))
  ;[0.2555 0.7775 1] Setup Option Buttons
  (`self.RemoveXrayROS`)
  (`self.UpdateCropBox_ROS`))

(event `LockMaterialTag`
  (params (Actor :type "Actor Object Reference"))
  (`/Engine/EditorBlueprintResources/StandardMacros.IsValid` Actor
    (:`Is Valid`
      (`KismetArrayLibrary.Array_Add` (`Actor.Tags` Actor) "Locked_XRAY"))))

(event `self.BindSaveGame`
  (params (PersistentUI :type "/Game/CollaborativeViewer/UMG/GameMenu/Persistent_ToolBar Object Reference"))
  ;[0.2555 0.7775 1] Binding Save Load SaveGame
  (add `/Game/CollaborativeViewer/UMG/GameMenu/Persistent_ToolBar.LoadState` PersistentUI (delegate `BindLoad`))
  (add `/Game/CollaborativeViewer/UMG/GameMenu/Persistent_ToolBar.SavingState` PersistentUI (delegate `BindSave`)))

(event `BindLoad`
  (params (SlotName :type String) (SaveGame :type "/Game/CollaborativeViewer/Blueprints/SaveGame/BP_Data_SaveGame Object Reference"))
  ;[0.2555 0.7775 1] Binding Save Load SaveGame
  (`self.LoadSaveGame` SlotName SaveGame))

(event `BindSave`
  (params (SlotName :type "String (by ref)"))
  ;[0.2555 0.7775 1] Binding Save Load SaveGame
  (`self.ToSaveGameROS` SlotName))

(event `RemoveLockMaterialTag`
  (params (Actor :type "Actor Object Reference"))
  (`/Engine/EditorBlueprintResources/StandardMacros.IsValid` Actor
    (:`Is Valid`
      (`KismetArrayLibrary.Array_RemoveItem` (`Actor.Tags` Actor) "Locked_XRAY"))))

(event `ApplyXray`
  (params (Actor :type "Actor Object Reference"))
  ;[0.2555 0.7775 1] ApplyXray
  (`/Engine/EditorBlueprintResources/StandardMacros.IsValid` Actor
    (:`Is Valid`
      (for _array_element (`Actor.K2_GetComponentsByClass` Actor "/Script/Engine.StaticMeshComponent")
        (`PrimitiveComponent.SetCollisionObjectType` _array_element "ECC_GameTraceChannel6")
        (for _index (range (`PrimitiveComponent.GetNumMaterials` _array_element))
          (`PrimitiveComponent.SetMaterial` _array_element _index "/Game/CollaborativeViewer/Blueprints/Commands/Xray/Materials/MI_Xray.MI_Xray"))))))

(event `ApplyXrayMTC`
  (params (NameTag :type String))
  (bind _actor (`/Game/CollaborativeViewer/Blueprints/ShareLibrary/CommonFunctions_CV.GetActorFromTag` NameTag))
  (bind _locked (`/Game/CollaborativeViewer/Blueprints/ShareLibrary/CommonFunctions_CV.Is Actor Locked With Tag` _actor))
  ;[0.2555 0.7775 1] ApplyXray
  (if (not _locked)
    (`self.LockMaterialTag` _actor)
    (bind _returnvalue (`GameplayStatics.GetActorOfClass` "/Game/CollaborativeViewer/Blueprints/Commands/Xray/BPs/XrayManager.XrayManager_C"))
    (`/Game/CollaborativeViewer/Blueprints/Commands/Xray/BPs/XrayManager.getMaterials` _returnvalue _actor)
    (`self.ApplyXray` _actor)))

(event `ApplyXray_ROS`
  (params (Actor :type "String (by ref)"))
  ;[0.2555 0.7775 1] ApplyXray
  (bind _locked (`/Game/CollaborativeViewer/Blueprints/ShareLibrary/CommonFunctions_CV.Is Actor Locked With Tag` (`/Game/CollaborativeViewer/Blueprints/ShareLibrary/CommonFunctions_CV.GetActorFromTag` Actor)))
  (if (not _locked)
    (`/Game/CollaborativeViewer/Blueprints/Commands/Xray/BPs/XrayManager.AddXrayActor` (`self.XrayManager`) Actor)
    (`self.ApplyXrayMTC` Actor)))

(event `RemoveXray`
  (params (XrayActors :type "Array of String") (MaterialsArrays :type "Array of /Game/CollaborativeViewer/Blueprints/Commands/Xray/BPs/XrayMaterialsArrays Structure (by ref)"))
  ;[0.2555 0.7775 1] Remove X Ray
  (for (_array_element _array_index) XrayActors
    (bind _outactors (`GameplayStatics.GetAllActorsWithTag` (`KismetStringLibrary.Conv_StringToName` _array_element)))
    (bind _output (`|GetArrayItem` _outactors))
    (`/Engine/EditorBlueprintResources/StandardMacros.IsValid` _output
      (:`Is Valid`
        (bind (_locked _sufix) (`/Game/CollaborativeViewer/Blueprints/ShareLibrary/CommonFunctions_CV.Is Actor Locked With Tag` _output "XRAY"))
        (if _locked
          (if _sufix
            (`self.RemoveLockMaterialTag` _output)
            (bind _output_materials (break `/Game/CollaborativeViewer/Blueprints/Commands/Xray/BPs/XrayMaterialsArrays` (`|GetArrayItem` MaterialsArrays _array_index)))
            (set `self.CurrentActorMaterials` _output_materials)
            (for _array_element_2 (`Actor.K2_GetComponentsByClass` _output "/Script/Engine.StaticMeshComponent")
              (`PrimitiveComponent.SetCollisionObjectType` _array_element_2 "ECC_WorldDynamic")
              (for _index (range (`PrimitiveComponent.GetNumMaterials` _array_element_2))
                (`PrimitiveComponent.SetMaterial` _array_element_2 _index (`|GetArrayItem` (`self.CurrentActorMaterials`) (`self.CurrentIndexMaterial`)))
                (`/Engine/EditorBlueprintResources/StandardMacros.IncrementInt` (`self.CurrentIndexMaterial`))))
            (set `self.CurrentIndexMaterial` 0)))))))

(event `UpdateCropBox_MTC`
  ;[0.2555 0.7775 1] UpdateExternal Actor
  (bind _returnvalue (`GameplayStatics.GetActorOfClass` "/Game/CollaborativeViewer/Blueprints/Commands/CropBox/BPs/BP_CropBox.BP_CropBox_C"))
  (`/Engine/EditorBlueprintResources/StandardMacros.IsValid` _returnvalue
    (:`Is Valid`
      (`/Game/CollaborativeViewer/Blueprints/Commands/CropBox/BPs/BP_CropBox.Update` _returnvalue))))

(event `UpdateCropBox_ROS`
  ;[0.2555 0.7775 1] UpdateExternal Actor
  (`self.UpdateCropBox_MTC`))

(event `RemoveXrayMTC`
  (params (XrayActors :type "Array of String") (MaterialsArrays :type "Array of /Game/CollaborativeViewer/Blueprints/Commands/Xray/BPs/XrayMaterialsArrays Structure"))
  ;[0.2555 0.7775 1] Remove X Ray
  (`self.RemoveXray` XrayActors MaterialsArrays))

(event `RemoveXrayROS`
  ;[0.2555 0.7775 1] Remove X Ray
  (bind _returnvalue (`GameplayStatics.GetActorOfClass` "/Game/CollaborativeViewer/Blueprints/Commands/Xray/BPs/XrayManager.XrayManager_C"))
  (`self.RemoveXrayMTC` (`/Game/CollaborativeViewer/Blueprints/Commands/Xray/BPs/XrayManager.XrayActors` _returnvalue) (`/Game/CollaborativeViewer/Blueprints/Commands/Xray/BPs/XrayManager.MaterialsArrays` _returnvalue))
  (`/Game/CollaborativeViewer/Blueprints/Commands/Xray/BPs/XrayManager.ClearXrayActors` _returnvalue))

(event `SetIsolateArrayActors`
  (params (HitActor :type "Actor Object Reference"))
  ;[0.2555 0.7775 1] Isolate X Ray
  (`/Engine/EditorBlueprintResources/StandardMacros.IsValid` HitActor
    (:`Is Valid`
      (bind _childrens (`self.GetallActorsOfHierarchy` HitActor))
      (bind _output_get (set `self.IsolatedActorArray` _childrens))
      (`KismetArrayLibrary.Array_RemoveItem` _output_get (`/Game/CollaborativeViewer/Blueprints/ShareLibrary/CommonFunctions_CV.GetCollabTag` HitActor)))))

(event `IsolateXrayMTC`
  (params (XrayActorsArray :type "Array of String (by ref)"))
  ;[0.2555 0.7775 1] Isolate X Ray
  (for _array_element XrayActorsArray
    (bind _actor (`/Game/CollaborativeViewer/Blueprints/ShareLibrary/CommonFunctions_CV.GetActorFromTag` _array_element))
    (bind _locked (`/Game/CollaborativeViewer/Blueprints/ShareLibrary/CommonFunctions_CV.Is Actor Locked With Tag` _actor))
    (if (not _locked)
      (`self.LockMaterialTag` _actor)
      (bind _returnvalue (`GameplayStatics.GetActorOfClass` "/Game/CollaborativeViewer/Blueprints/Commands/Xray/BPs/XrayManager.XrayManager_C"))
      (`/Game/CollaborativeViewer/Blueprints/Commands/Xray/BPs/XrayManager.getMaterials` _returnvalue _actor)
      (`self.ApplyXray` _actor))))

(event `IsolateXrayROS`
  (params (XrayActorsArray :type "Array of String (by ref)"))
  ;[0.2555 0.7775 1] Isolate X Ray
  (bind _returnvalue (`GameplayStatics.GetActorOfClass` "/Game/CollaborativeViewer/Blueprints/Commands/Xray/BPs/XrayManager.XrayManager_C"))
  (`/Game/CollaborativeViewer/Blueprints/Commands/Xray/BPs/XrayManager.AddArrayXrayActor` _returnvalue XrayActorsArray)
  (`self.IsolateXrayMTC` XrayActorsArray))

(event `LoadSaveGame`
  (params (SlotName :type String) (SaveGame :type "/Game/CollaborativeViewer/Blueprints/SaveGame/BP_Data_SaveGame Object Reference"))
  ;[1 0.6656 0.1995] SaveGame
  (`self.RemoveXrayROS`)
  (for _array_element (`/Game/CollaborativeViewer/Blueprints/SaveGame/BP_Data_SaveGame.XrayObjectNames` SaveGame)
    (`self.ApplyXray_ROS` _array_element)))

(event `ToSaveGameMTC`
  (params (SlotName :type String) (XrayActors :type "Array of String (by ref)"))
  ;[1 0.6656 0.1995] SaveGame
  (bind _asbp_collab_v_player_controller (cast `/Game/CollaborativeViewer/Blueprints/PlayerController/BP_Collab_V_PlayerController` (`GameplayStatics.GetPlayerController` 0)))
  (bind _datasavegame (`/Game/CollaborativeViewer/Blueprints/PlayerController/BP_Collab_V_PlayerController.DataSaveGame` _asbp_collab_v_player_controller))
  (set `/Game/CollaborativeViewer/Blueprints/SaveGame/BP_Data_SaveGame.XrayObjectNames` XrayActors _datasavegame)
  (`/Engine/EditorBlueprintResources/StandardMacros.IsValid` _datasavegame
    (:`Is Valid`
      (`GameplayStatics.SaveGameToSlot` _datasavegame SlotName))))

(event `ToSaveGameROS`
  (params (SlotName :type String))
  ;[1 0.6656 0.1995] SaveGame
  (bind _returnvalue (`GameplayStatics.GetActorOfClass` "/Game/CollaborativeViewer/Blueprints/Commands/Xray/BPs/XrayManager.XrayManager_C"))
  (`self.ToSaveGameMTC` SlotName (`/Game/CollaborativeViewer/Blueprints/Commands/Xray/BPs/XrayManager.XrayActors` _returnvalue)))

(fn `GetallActorsOfHierarchy`
  (params (CurrentHitActor :type "Actor Object Reference"))
  (returns (Childrens :type "Array of String"))
  (locals (CollabActorsTag_L :type "Array of String"))
  (bind _lasthierarchyparent (`/Game/CollaborativeViewer/Blueprints/ShareLibrary/CommonFunctions_CV.GetHierarchyLastParent` CurrentHitActor))
  (bind _childrens (`/Game/CollaborativeViewer/Blueprints/ShareLibrary/CommonFunctions_CV.GetAttachedActors` _lasthierarchyparent))
  (for _array_element _childrens
    (bind _locked (`/Game/CollaborativeViewer/Blueprints/ShareLibrary/CommonFunctions_CV.Is Actor Locked With Tag` _array_element))
    (if (not _locked)
      (bind _actorname (`/Game/CollaborativeViewer/Blueprints/ShareLibrary/CommonFunctions_CV.GetCollabTag` _array_element))
      (if (not (`KismetStringLibrary.IsEmpty` _actorname))
        (`KismetArrayLibrary.Array_AddUnique` (`local.CollabActorsTag_L`) _actorname))))
  (return (`local.CollabActorsTag_L`)))

(fn `OnRep_CurrentActorMaterials`)