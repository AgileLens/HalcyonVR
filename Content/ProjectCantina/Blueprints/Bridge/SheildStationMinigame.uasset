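; Shield station minigame on the bridge where the player rotates a blocker to protect a ship from incoming blaster bolts.
; Activation starts a round through a DoOnce; each timeline-driven bolt flies inward from a random angle while interaction input turns the blocker pivot.
; Blocks score and fire another bolt; a ship hit saves any high score and re-arms activation.
; Looping timers spin the score text before play, then face it toward the player.
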(event `self.ReceiveBeginPlay`
  (bind _returnvalue (`KismetSystemLibrary.K2_SetTimerDelegate` (delegate `RotateHighscore`) 0.02 true)))

(event `End Game`
  (`PrimitiveComponent.SetMaterial` (`self.Ship`) 0 "/Game/ProjectCantina/Materials/Atrium/MI_Blue.MI_Blue")
  (`|ExecutionSequence`
    (:`then_0`
      (`KismetSystemLibrary.K2_PauseTimerHandle` (stale `Game Start` _returnvalue))
      (if (> (`self.ScoreCount`) (`self.HighScore`))
        (set `self.HighScore` (`self.ScoreCount`)))
      (`TextRenderComponent.K2_SetText` (`self.SCORE1`) (`KismetTextLibrary.Conv_IntToText` (`self.HighScore`)))
      (`TextRenderComponent.K2_SetText` (`self.SCORE`) "HIGH SCORE")
      (set `self.ScoreCount` 0))
    (:`then_1`
      (goto _label :!via `Reset`))))

(event `RotateHighscore`
  (`SceneComponent.K2_AddLocalRotation` (`self.TEXT`) (`KismetMathLibrary.MakeRotator` 0.0 0.0 1.0) false false))

(event `Game Start`
  (`TextRenderComponent.K2_SetText` (`self.SCORE`) "YOUR SCORE")
  (`KismetSystemLibrary.K2_PauseTimerHandle` (stale `self.ReceiveBeginPlay` _returnvalue))
  (`self.Shoot`)
  (bind _returnvalue (`KismetSystemLibrary.K2_SetTimerDelegate` (delegate `RotateScoreTowardPlayer`) 0.02 true)))

(event `/Game/GDXR_VR_Template/Blueprints/Interfaces/BPI_PlayerInteractions.Activation`
  (params (State :type Boolean))
  (if State
    (`/Engine/EditorBlueprintResources/StandardMacros.DoOnce` false :!label _label
      (:`Completed`
        (`self.Game Start`)))))

(event `RotateScoreTowardPlayer`
  (bind (_returnvalue_x _returnvalue_y) (`KismetMathLibrary.BreakVector` (`SceneComponent.K2_GetComponentLocation` (`self.TEXT`))))
  (bind (_returnvalue_x_2 _returnvalue_y_2) (`KismetMathLibrary.BreakVector` (`self.K2_GetActorLocation` (`self.Pawn`))))
  (bind (_returnvalue_roll _returnvalue_pitch _returnvalue_yaw) (`KismetMathLibrary.BreakRotator` (`KismetMathLibrary.FindLookAtRotation` (`KismetMathLibrary.MakeVector` _returnvalue_x _returnvalue_y) (`KismetMathLibrary.MakeVector` _returnvalue_x_2 _returnvalue_y_2))))
  (`SceneComponent.K2_SetWorldRotation` (`self.TEXT`) (`KismetMathLibrary.MakeRotator` 0.0 0.0 _returnvalue_yaw) false false))

(event `Shoot`
  (`SceneComponent.SetVisibility` (`self.Bolt`) true false)
  (`SceneComponent.K2_SetRelativeRotation` (`self.Scene`) (`KismetMathLibrary.MakeRotator` 0.0 0.0 (`KismetMathLibrary.RandomFloatInRange` 0.0 360.0)) false false)
  (bind (_direction _newtrack_0) (`Timeline|Animate Bolt` :!via `PlayFromStart` :!label _label_2)
    (:`Update`
      (`SceneComponent.K2_SetRelativeLocation` (`self.Bolt`) (`KismetMathLibrary.MakeVector` (`KismetMathLibrary.Lerp` 70.0 0.0 _newtrack_0)) false false))))

(event `/Game/GDXR_VR_Template/Blueprints/Interfaces/BPI_PlayerInteractions.CurrentlyInteracting`
  (params (RequiredFloat :type "Float (double-precision)") (RequiredBoolean :type Boolean) (RequiredVector :type "Vector Structure"))
  (`SceneComponent.K2_AddLocalRotation` (`self.Scene2`) (`KismetMathLibrary.MakeRotator` 0.0 0.0 (`KismetMathLibrary.FClamp` (* RequiredVector_Y 0.5) -4.0 4.0)) false false))

(event `self.ReceiveTick`
  (params (DeltaSeconds :type "Float (single-precision)")))

(event `self.Bolt.OnComponentBeginOverlap`
  (params (OverlappedComponent :type "PrimitiveComponent Object Reference") (OtherActor :type "Actor Object Reference") (OtherComp :type "PrimitiveComponent Object Reference") (OtherBodyIndex :type Integer) (bFromSweep :type Boolean) (SweepResult :type "HitResult Structure (by ref)"))
  (bind _blocker (`self.Blocker`))
  (bind _bolt (`self.Bolt`))
  (if (== OtherComp (`self.Ship`))
    (`SceneComponent.SetVisibility` _bolt false false)
    (`PrimitiveComponent.SetMaterial` (`self.Ship`) 0 "/Game/ProjectCantina/Materials/Atrium/MI_Blaster.MI_Blaster")
    (`self.End Game`)
    (elif (== OtherComp (`self.Blocker`))
      (`SceneComponent.SetVisibility` _bolt false false)
      (`|ExecutionSequence`
        (:`then_0`
          (`PrimitiveComponent.SetMaterial` _blocker 0 "/Game/ProjectCantina/Materials/Atrium/MI_Blaster.MI_Blaster")
          (`KismetSystemLibrary.Delay` 1.0)
          (`PrimitiveComponent.SetMaterial` _blocker 0 "/Game/ProjectCantina/Materials/Atrium/MI_light_gray_plastic.MI_light_gray_plastic"))
        (:`then_1`
          (goto _label_2 :!via `Stop`))
        (:`then_2`
          (bind _output_get (set `self.ScoreCount` (+ (`self.ScoreCount`) 1)))
          (`TextRenderComponent.K2_SetText` (`self.SCORE1`) (`KismetTextLibrary.Conv_IntToText` _output_get))
          (`self.Shoot`))))))

(fn `UserConstructionScript`)