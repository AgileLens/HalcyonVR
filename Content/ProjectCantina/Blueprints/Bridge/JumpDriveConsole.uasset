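; Bridge console with a VR-grabbable lever that triggers the hyperspace jump level sequence, or occasionally just a hyperdrive trouble sound.
; While either grab component is held, a looping timer pitches the lever toward the motion controller within clamped limits, firing once past a threshold.
; Releasing both grabs eases the lever back and re-arms it.
; An Interact event instead animates the pull with a timeline, then reverses and resets after a delay.
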(event `self.C_GrabComponent1.FirstHandGrabbed`
  (params (`Motion Controller` :type "MotionControllerComponent Object Reference") (SkeltalMeshHand :type "SkeletalMeshComponent Object Reference") (`Motion Controller Aim` :type "MotionControllerComponent Object Reference"))
  (set `self.Motion Controller` `Motion Controller`)
  (`/Game/TemplateContent/Blueprints/C_GrabComponent.Snap Skeletal Hand` (`self.C_GrabComponent`) (`self.Motion Controller`) (`self.SnapHand`) (`self.SnapHand`) null)
  (`self.SwitchLeverHandGrabbed` `Motion Controller`)
  (`KismetSystemLibrary.K2_SetTimerDelegate` (delegate `Update Rotation`) 0.02 true :!label _label)
  ;[1 1 1] Snap Hand To Actor Re using the snap hand child for both left and right
  (`/Game/TemplateContent/Blueprints/C_GrabComponent.Snap Skeletal Hand` (`self.C_GrabComponent`) (`self.Motion Controller`) (`self.SnapHand`) (`self.SnapHand`) (stale `self.C_GrabComponent.FirstHandGrabbed` SkeltalMeshHand)))

(event `/Game/ProjectCantina/Blueprints/BPI_PawnCommunication.Interact`
  (`|ExecutionSequence`
    (:`then_0`
      (`/Engine/EditorBlueprintResources/StandardMacros.DoOnce` false :!label _label_2
        (:`Completed`
          (bind (_direction _newtrack_0) (`Timeline|Timeline` :!via `PlayFromStart` :!label _label_3)
            (:`Update`
              (`SceneComponent.K2_SetRelativeRotation` (`self.Switchbase`) (`KismetMathLibrary.MakeRotator` 0.0 (`KismetMathLibrary.Lerp` 0.0 90.0 _newtrack_0)) true false))
            (:`Finished`
              (if (> (> _newtrack_0 0.9) 0)
                (if (== (`KismetMathLibrary.RandomIntegerInRange` 0 12) 11) :!label _label_4
                  (`GameplayStatics.PlaySoundAtLocation` "/Game/Audio/hyperdriveTrouble_Cue.hyperdriveTrouble_Cue" (`SceneComponent.K2_GetComponentLocation` (`self.Console`)) (struct) 1.0 1.0 0.0 null null null null)
                  (else
                    (bind (_outactor _returnvalue) (`LevelSequencePlayer.CreateLevelSequencePlayer` "/Game/ProjectCantina/Sequences/LS_Hyperspace.LS_Hyperspace"))
                    (`MovieSceneSequencePlayer.Play` _returnvalue)))))))))
    (:`then_1`
      (`KismetSystemLibrary.Delay` 4.0)
      (goto _label_2 :!via `Reset`))
    (:`then_2`
      (`KismetSystemLibrary.Delay` 4.0)
      (goto _label_3 :!via `ReverseFromEnd`))))

(event `self.C_GrabComponent.FirstHandGrabbed`
  (params (`Motion Controller` :type "MotionControllerComponent Object Reference") (SkeltalMeshHand :type "SkeletalMeshComponent Object Reference") (`Motion Controller Aim` :type "MotionControllerComponent Object Reference"))
  (set `self.Motion Controller` `Motion Controller`)
  (`self.SwitchLeverHandGrabbed` `Motion Controller`)
  (goto _label))

(event `Update Rotation`
  (bind _switchbase (`self.Switchbase`))
  (bind (_relativerotation_roll _relativerotation_pitch) (`KismetMathLibrary.BreakRotator` (`SceneComponent.RelativeRotation` _switchbase)))
  (bind (_returnvalue_roll _returnvalue_pitch) (`KismetMathLibrary.BreakRotator` (`KismetMathLibrary.FindLookAtRotation` (`SceneComponent.K2_GetComponentLocation` (`self.Switchbase`)) (`SceneComponent.K2_GetComponentLocation` (stale `self.C_GrabComponent.FirstHandGrabbed` `Motion Controller`)))))
  (`SceneComponent.K2_SetRelativeRotation` _switchbase (`KismetMathLibrary.MakeRotator` 0.0 (`KismetMathLibrary.ClampAngle` _returnvalue_pitch 0.0 80.0)) true false)
  (if (> _relativerotation_pitch 70.0)
    (`/Engine/EditorBlueprintResources/StandardMacros.DoOnce` false :!label _label_5
      (:`Completed`
        (goto _label_4)))))

(event `self.C_GrabComponent.FirstHandDropped`
  (params (`Original Hand Location` :type "Transform Structure") (`Motion Controller` :type "MotionControllerComponent Object Reference") (`Skeletal Mesh Hand` :type "SkeletalMeshComponent Object Reference"))
  (bind _switchbase (`self.Switchbase`))
  (bind (_relativerotation_roll _relativerotation_pitch _relativerotation_yaw) (`KismetMathLibrary.BreakRotator` (`SceneComponent.RelativeRotation` _switchbase)))
  (if (not (`/Game/TemplateContent/Blueprints/C_GrabComponent.bIsHeld` (`self.C_GrabComponent1`)))
    (`KismetSystemLibrary.K2_PauseTimer` null "Update Rotation" :!label _label_6)
    (set `self.Motion Controller` null)
    (set `self.Relative Rotation Z (Yaw)` _relativerotation_yaw)
    (bind (_direction _newtrack_0) (`Timeline|RotBack` :!via `PlayFromStart`)
      (:`Update`
        (`SceneComponent.K2_SetRelativeRotation` _switchbase (`KismetMathLibrary.MakeRotator` 0.0 (`KismetMathLibrary.Lerp` (`self.Relative Rotation Z (Yaw)`) 0.0 _newtrack_0)) true false))
      (:`Finished`
        (goto _label_5 :!via `Reset`)))))

(event `self.C_GrabComponent1.FirstHandDropped`
  (params (`Original Hand Location` :type "Transform Structure") (`Motion Controller` :type "MotionControllerComponent Object Reference") (`Skeletal Mesh Hand` :type "SkeletalMeshComponent Object Reference"))
  (if (not (`/Game/TemplateContent/Blueprints/C_GrabComponent.bIsHeld` (`self.C_GrabComponent`)))
    (goto _label_6)))

(fn `UserConstructionScript`)