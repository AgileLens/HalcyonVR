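; BP_SheildJoyStick is a grabbable bridge joystick that drives an assigned ActorToControl through interaction messages.
; On first grab it snaps the hand, sends activation and starts a looping timer.
; Each tick pitches the stick toward the motion controller using look-at dot products, clamping the step but applying no roll, then sends negated roll and pitch.
; Release calls a timer pause by function name and recenters the stick.
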(event `self.C_GrabComponent.FirstHandGrabbed`
  (params (`Motion Controller` :type "MotionControllerComponent Object Reference") (SkeltalMeshHand :type "SkeletalMeshComponent Object Reference") (`Motion Controller Aim` :type "MotionControllerComponent Object Reference"))
  (`KismetSystemLibrary.PrintString` "GRABBBBED")
  (set `self.Motion Controller` `Motion Controller`)
  (message `/Game/TemplateContent/Blueprints/Interfaces/BPI_PlayerInteractions.Activation` (`self.ActorToControl`) true)
  (`KismetSystemLibrary.K2_SetTimerDelegate` (delegate `Update Position`) 0.02 true)
  (`/Game/TemplateContent/Blueprints/C_GrabComponent.Snap Skeletal Hand` (`self.C_GrabComponent`) (`self.Motion Controller`) (`self.SnapHand`) (`self.SnapHand`) SkeltalMeshHand))

(event `Update Position`
  (bind _joystick (`self.Joystick`))
  (bind _joystick_2 (`self.Joystick`))
  (bind _joystick_3 (`self.Joystick`))
  (bind (_relativerotation_roll _relativerotation_pitch) (`KismetMathLibrary.BreakRotator` (`SceneComponent.RelativeRotation` _joystick_2)))
  (bind (_returnvalue_roll _returnvalue_pitch) (`KismetMathLibrary.BreakRotator` (`KismetMathLibrary.MakeRotator` (* (`KismetMathLibrary.Dot_VectorVector` (`KismetMathLibrary.Conv_RotatorToVector` (`KismetMathLibrary.FindLookAtRotation` (`SceneComponent.K2_GetComponentLocation` _joystick_3) (`SceneComponent.K2_GetComponentLocation` (`self.Motion Controller`)))) (`KismetMathLibrary.GetRightVector` (`SceneComponent.K2_GetComponentRotation` _joystick_3))) 10.0) (* (`KismetMathLibrary.Dot_VectorVector` (`KismetMathLibrary.Conv_RotatorToVector` (`KismetMathLibrary.FindLookAtRotation` (`SceneComponent.K2_GetComponentLocation` _joystick) (`SceneComponent.K2_GetComponentLocation` (`self.Motion Controller`)))) (* (`KismetMathLibrary.GetForwardVector` (`SceneComponent.K2_GetComponentRotation` _joystick)) -1.0)) 10.0))))
  ;[1 1 1] Calculate left Right Position
  (`SceneComponent.K2_AddRelativeRotation` _joystick_2 (`KismetMathLibrary.MakeRotator` 0.0 (`KismetMathLibrary.FClamp` _returnvalue_pitch -20.0 20.0)) false false)
  (message `/Game/TemplateContent/Blueprints/Interfaces/BPI_PlayerInteractions.CurrentlyInteracting` (`self.ActorToControl`) 0.0 false (`KismetMathLibrary.MakeVector` (* _relativerotation_roll -1.0) (* _relativerotation_pitch -1.0))))

(event `self.C_GrabComponent.FirstHandDropped`
  (params (`Original Hand Location` :type "Transform Structure") (`Motion Controller` :type "MotionControllerComponent Object Reference") (`Skeletal Mesh Hand` :type "SkeletalMeshComponent Object Reference"))
  (`KismetSystemLibrary.K2_PauseTimer` null "Update Position")
  (`SceneComponent.K2_SetRelativeRotation` :`self` (`self.Joystick`)))

(fn `UserConstructionScript`)