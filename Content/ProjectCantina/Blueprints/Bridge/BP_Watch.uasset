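; Bridge trigger volume that plays audio as the player and captain (BP_Kendra) enter.
; Player entry fires a one-shot intro, ambient hum and delayed systems-up cue; captain entry fires a delayed announcement, also one-shot.
; When the player leaves, a valid hum stops and a 20-second timer starts to reset both DoOnce gates.
; Player re-entry pauses that timer, so returning early replays neither the cues nor the hum.
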(event `self.ReceiveBeginPlay`
  (bind _returnvalue (`GameplayStatics.GetActorOfClass` "/Game/MetaHumans/Captain_Keevan/BP_Kendra.BP_Kendra_C"))
  (set `self.Captain` _returnvalue))

(event `self.Box.OnComponentBeginOverlap`
  (params (OverlappedComponent :type "PrimitiveComponent Object Reference") (OtherActor :type "Actor Object Reference") (OtherComp :type "PrimitiveComponent Object Reference") (OtherBodyIndex :type Integer) (bFromSweep :type Boolean) (SweepResult :type "HitResult Structure (by ref)"))
  (bind _returnvalue (`SceneComponent.K2_GetComponentLocation` (`self.SoundLocation`)))
  (if (== OtherActor (`GameplayStatics.GetPlayerPawn` 0))
    (`|ExecutionSequence`
      (:`then_0`
        (`/Engine/EditorBlueprintResources/StandardMacros.DoOnce` false :!label _label
          (:`Completed`
            (`GameplayStatics.PlaySoundAtLocation` "/Game/Audio/Watcher_Audio/Intro_Cue.Intro_Cue" _returnvalue (struct) 1.0 1.0 0.0 null null null null)
            (bind _returnvalue_2 (`GameplayStatics.SpawnSoundAtLocation` "/Game/Audio/Spaceship_in_Flight_Ambience_with_Low_Phased_Hum_and_Rumble_Cue.Spaceship_in_Flight_Ambience_with_Low_Phased_Hum_and_Rumble_Cue" _returnvalue (struct) 1.0 1.0 0.0 null null))
            (set `self.SpaceHum` _returnvalue_2)
            (`KismetSystemLibrary.Delay` 5.0)
            (`GameplayStatics.PlaySoundAtLocation` "/Game/Audio/Watcher_Audio/Bringing_Systems_Up_Cue.Bringing_Systems_Up_Cue" _returnvalue (struct) 1.0 1.0 0.0 null null null null))))
      (:`then_1`
        (`KismetSystemLibrary.K2_PauseTimerHandle` (stale `self.Box.OnComponentEndOverlap` _returnvalue))))
    (elif (== (`self.Captain`) OtherActor)
      (`/Engine/EditorBlueprintResources/StandardMacros.DoOnce` false :!label _label_2
        (:`Completed`
          (`KismetSystemLibrary.Delay` 4.0)
          (`GameplayStatics.PlaySoundAtLocation` "/Game/Audio/Watcher_Audio/Captain_On_The_Bridge_Cue.Captain_On_The_Bridge_Cue" _returnvalue (struct) 1.0 1.0 0.0 null null null null))))))

(event `UnlockWatch`
  (`|ExecutionSequence`
    (:`then_0`
      (goto _label :!via `Reset`))
    (:`then_1`
      (goto _label_2 :!via `Reset`))))

(event `self.Box.OnComponentEndOverlap`
  (params (OverlappedComponent :type "PrimitiveComponent Object Reference") (OtherActor :type "Actor Object Reference") (OtherComp :type "PrimitiveComponent Object Reference") (OtherBodyIndex :type Integer))
  (bind _spacehum (`self.SpaceHum`))
  (if (== OtherActor (`GameplayStatics.GetPlayerPawn` 0))
    (`/Engine/EditorBlueprintResources/StandardMacros.IsValid` _spacehum
      (:`Is Valid`
        (`AudioComponent.Stop` _spacehum)
        (bind _returnvalue (`KismetSystemLibrary.K2_SetTimerDelegate` (delegate `UnlockWatch`) 20.0))))))

(fn `UserConstructionScript`)