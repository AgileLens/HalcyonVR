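; BP_SwitchExample is an example interactable actor that other actors drive through the BPI_PlayerInteractions interface.
; Activation swaps its Sphere's material between green and the basic shape material according to the State flag.
; CurrentlyInteracting moves the actor one unit along X and Y, using only the sign of the supplied vector's components to pick each direction.
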(event `self.Activation`
  (params (State :type Boolean))
  (bind _sphere (`self.Sphere`))
  ;[1 1 1] Contains the blueprint interface (BPI_PlayerInteractions) and allows other actors with a refrence to tell this actor what it can do.
  (if State
    (`PrimitiveComponent.SetMaterial` _sphere 0 "/AnimationSharing/AnimSharingGreen.AnimSharingGreen")
    (else
      (`PrimitiveComponent.SetMaterial` _sphere 0 "/Engine/BasicShapes/BasicShapeMaterial.BasicShapeMaterial"))))

(event `self.CurrentlyInteracting`
  (params (RequiredFloat :type "Float (double-precision)") (RequiredBoolean :type Boolean) (RequiredVector :type "Vector Structure"))
  (bind (_returnvalue_x _returnvalue_y) (`KismetMathLibrary.BreakVector` (`self.K2_GetActorLocation`)))
  (`self.K2_SetActorLocation` (`KismetMathLibrary.MakeVector` (+ _returnvalue_x (`KismetMathLibrary.SelectFloat` 1.0 -1.0 (> RequiredVector_X 0.0))) (+ _returnvalue_y (`KismetMathLibrary.SelectFloat` 1.0 -1.0 (> RequiredVector_Y 0.0))))))

(fn `UserConstructionScript`)