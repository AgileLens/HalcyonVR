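; Grabbable VR training lightsaber whose blade extends and retracts when the holding hand presses interact.
; While held, it binds ToggleBlade to the VR_GameInstance grabbed-item interact event, then unbinds and retracts on drop.
; The Sheath timeline scales the blade's Z to open or close it, also starting retracted on BeginPlay.
; DoOnce gates, reset when the timeline finishes, limit ignite and retract haptics and sounds sent through the game instance.
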(event `self.GrabComponent.OnGrabbed`
  (bind _asvr_game_instance (cast `/Game/GDXR_VR_Template/Blueprints/VR_GameInstance` (`GameplayStatics.GetGameInstance`)))
  (add `/Game/GDXR_VR_Template/Blueprints/VR_GameInstance.GrabbedItemInteract` _asvr_game_instance (delegate `ToggleBlade`)))

(event `ToggleBlade`
  (params (RightHand :type Boolean))
  (bind _returnvalue (`self.K2_GetActorLocation`))
  (bind _returnvalue_2 (`/Game/VRTemplate/Blueprints/GrabComponent.GetHeldByHand` (`self.GrabComponent`)))
  (bind _returnvalue_3 (`|EnumEquality` (`/Game/VRTemplate/Blueprints/GrabComponent.GetHeldByHand` (`self.GrabComponent`)) "Right"))
  (if RightHand
    (if (`|EnumEquality` _returnvalue_2 "Right")
      (if (== (stale _newtrack_0) 0.0) :!label _label
        (`|ExecutionSequence` :!label _label_2
          (:`then_0`
            (bind (_direction _newtrack_0) (`Timeline|Sheath` :!label _label_3)
              (:`Update`
                (`SceneComponent.SetRelativeScale3D` (`self.Blade`) (`KismetMathLibrary.MakeVector` 334.913423 334.913423 (`KismetMathLibrary.Lerp` 1.0 268.635402 _newtrack_0))))
              (:`Finished`
                (`|ExecutionSequence`
                  (:`then_0`
                    (goto _label_4 :!via `Reset`))
                  (:`then_1`
                    (goto _label_5 :!via `Reset`))))))
          (:`then_1`
            (`/Engine/EditorBlueprintResources/StandardMacros.DoOnce` false :!label _label_4
              (:`Completed`
                (`/Game/GDXR_VR_Template/Blueprints/VR_GameInstance.PlayHaptic` (`self.As VR Game Instance`) _returnvalue_3 "/Game/ProjectCantina/Haptics/Ignite.Ignite" "/Game/ProjectCantina/Audio/Ignite__Cue.Ignite__Cue" _returnvalue)))))
        (else
          (`|ExecutionSequence`
            (:`then_0`
              (goto _label_3 :!via `Reverse`))
            (:`then_1`
              (`/Engine/EditorBlueprintResources/StandardMacros.DoOnce` false :!label _label_5
                (:`Completed`
                  (`/Game/GDXR_VR_Template/Blueprints/VR_GameInstance.PlayHaptic` (`self.As VR Game Instance`) _returnvalue_3 "/Game/ProjectCantina/Haptics/Retract.Retract" "/Game/ProjectCantina/Audio/Retract__Cue.Retract__Cue" _returnvalue))))))))
    (elif (`|EnumEquality` _returnvalue_2 "Left")
      (goto _label))))

(event `OpenBlade`
  (goto _label_2))

(event `CloseBlade`
  (goto _label_3 :!via `Reverse`))

(event `self.GrabComponent.OnDropped`
  (bind _asvr_game_instance (cast `/Game/GDXR_VR_Template/Blueprints/VR_GameInstance` (`GameplayStatics.GetGameInstance`)))
  (remove `/Game/GDXR_VR_Template/Blueprints/VR_GameInstance.GrabbedItemInteract` _asvr_game_instance (delegate `ToggleBlade`))
  (`self.CloseBlade` :!label _label_6))

(event `self.ReceiveBeginPlay`
  (bind _asvr_game_instance (cast `/Game/GDXR_VR_Template/Blueprints/VR_GameInstance` (`GameplayStatics.GetGameInstance`)))
  (set `self.As VR Game Instance` _asvr_game_instance)
  (goto _label_6))

(fn `UserConstructionScript`)