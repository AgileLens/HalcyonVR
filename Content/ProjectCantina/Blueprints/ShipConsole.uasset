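; Ship console with physical buttons that navigates start, main, travel and confirm screens to load one of four levels.
; ScreenNumber acts as a state machine deciding what buttons 1–4 do, with screens switched by toggling component visibility.
; Halcyon pawn overlaps trigger per-button timelines that move and light the button, using DoOnce gates to fire each action once per press.
; Buttons 5–7 only animate and light up, with no screen action.
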(event `self.ReceiveBeginPlay`
  (`self.DisableAllScreen`)
  (`self.ShowStartScreen`)
  (bind _returnvalue (`GameplayStatics.GetActorOfClass` "/Game/ProjectCantina/Blueprints/BP_HalcyonPawn.BP_HalcyonPawn_C"))
  (set `self.PawnRef` _returnvalue))

(event `Button1Pressed`
  (switch `int` (`self.ScreenNumber`)
    (:`0`
      (`self.DisableAllScreen`)
      (`self.ShowMainScreen`)
      (set `self.ScreenNumber` 1))
    (:`1`
      (`self.DisableAllScreen`)
      (`self.ShowTravelScreen`)
      (set `self.ScreenNumber` 2))
    (:`2`
      (`self.DisableAllScreen`)
      (`self.ShowConfirmScreen`)
      (set `self.ScreenNumber` 3)
      (set `self.Selected Level` "DiningRoom"))
    (:`3`
      (`GameplayStatics.OpenLevel` (`self.Selected Level`)))))

(event `Button2Pressed`
  (switch `int` (`self.ScreenNumber`)
    (:`2`
      (`self.DisableAllScreen`)
      (`self.ShowConfirmScreen`)
      (set `self.ScreenNumber` 3)
      (set `self.Selected Level` "ClimateSim"))
    (:`3`
      (`self.DisableAllScreen`)
      (`self.ShowTravelScreen`)
      (set `self.ScreenNumber` 2))))

(event `Button3pressed`
  (switch `int` (`self.ScreenNumber`)
    (:`2`
      (`self.DisableAllScreen`)
      (`self.ShowConfirmScreen`)
      (set `self.ScreenNumber` 3)
      (set `self.Selected Level` "BedRoom"))))

(event `Button4Pressed`
  (switch `int` (`self.ScreenNumber`)
    (:`2`
      (`self.DisableAllScreen`)
      (`self.ShowConfirmScreen`)
      (set `self.ScreenNumber` 3)
      (set `self.Selected Level` "MainHall"))))

(event `self.Box1.OnComponentBeginOverlap`
  (params (OverlappedComponent :type "PrimitiveComponent Object Reference") (OtherActor :type "Actor Object Reference") (OtherComp :type "PrimitiveComponent Object Reference") (OtherBodyIndex :type Integer) (bFromSweep :type Boolean) (SweepResult :type "HitResult Structure (by ref)"))
  (bind _buttontop1 (`self.ButtonTop1`))
  (bind _pointlight (`self.PointLight`))
  ;[1 1 1] Button Animations (cant collapse because of timelines)
  (if (== OtherActor (`self.PawnRef`))
    (`/Engine/EditorBlueprintResources/StandardMacros.DoOnce` false :!label _label
      (:`Completed`
        (bind (_direction _newtrack_0) (`Timeline|ButtonTimeline01` :!via `PlayFromStart`)
          (:`Update`
            (`SceneComponent.K2_SetRelativeLocation` (`self.BottonPivot1`) (`KismetMathLibrary.VLerp` (0.0 0.0 0.0) (0.231025 0.0 -0.171261) _newtrack_0) false false)
            (if (< _newtrack_0 0.2)
              (`/Engine/EditorBlueprintResources/StandardMacros.DoOnce` false :!label _label_2
                (:`Completed`
                  (`PrimitiveComponent.SetMaterial` _buttontop1 0 "/Game/ProjectCantina/Materials/Console/ButtonMat.ButtonMat")
                  (`SceneComponent.SetVisibility` _pointlight true false)
                  (`self.Button1Pressed`)))))
          (:`Finished`
            (`|ExecutionSequence`
              (:`then_0`
                (`PrimitiveComponent.SetMaterial` _buttontop1 0 "/Game/ProjectCantina/Materials/Console/HalcyonTextureSheet_Mat.HalcyonTextureSheet_Mat")
                (`SceneComponent.SetVisibility` _pointlight false false)
                (`|ExecutionSequence`
                  (:`then_0`
                    (goto _label :!via `Reset`))
                  (:`then_1`
                    (goto _label_2 :!via `Reset`)))))))))))

(event `self.Box2.OnComponentBeginOverlap`
  (params (OverlappedComponent :type "PrimitiveComponent Object Reference") (OtherActor :type "Actor Object Reference") (OtherComp :type "PrimitiveComponent Object Reference") (OtherBodyIndex :type Integer) (bFromSweep :type Boolean) (SweepResult :type "HitResult Structure (by ref)"))
  (bind _buttontop2 (`self.ButtonTop2`))
  (bind _pointlight2 (`self.PointLight2`))
  ;[1 1 1] Button Animations (cant collapse because of timelines)
  (if (== OtherActor (`self.PawnRef`))
    (`/Engine/EditorBlueprintResources/StandardMacros.DoOnce` false :!label _label_3
      (:`Completed`
        (bind (_direction _newtrack_0) (`Timeline|Timeline` :!via `PlayFromStart`)
          (:`Update`
            (`SceneComponent.K2_SetRelativeLocation` (`self.BottonPivot2`) (`KismetMathLibrary.VLerp` (0.0 0.0 0.0) (0.231025 0.0 -0.171261) _newtrack_0) false false)
            (if (< _newtrack_0 0.2)
              (`/Engine/EditorBlueprintResources/StandardMacros.DoOnce` false :!label _label_4
                (:`Completed`
                  (`PrimitiveComponent.SetMaterial` _buttontop2 0 "/Game/ProjectCantina/Materials/Console/ButtonMat.ButtonMat")
                  (`SceneComponent.SetVisibility` _pointlight2 true false)
                  (`self.Button2Pressed`)))))
          (:`Finished`
            (`|ExecutionSequence`
              (:`then_0`
                (`PrimitiveComponent.SetMaterial` _buttontop2 0 "/Game/ProjectCantina/Materials/Console/HalcyonTextureSheet_Mat.HalcyonTextureSheet_Mat")
                (`SceneComponent.SetVisibility` _pointlight2 false false)
                (`|ExecutionSequence`
                  (:`then_0`
                    (goto _label_3 :!via `Reset`))
                  (:`then_1`
                    (goto _label_4 :!via `Reset`)))))))))))

(event `self.Box3.OnComponentBeginOverlap`
  (params (OverlappedComponent :type "PrimitiveComponent Object Reference") (OtherActor :type "Actor Object Reference") (OtherComp :type "PrimitiveComponent Object Reference") (OtherBodyIndex :type Integer) (bFromSweep :type Boolean) (SweepResult :type "HitResult Structure (by ref)"))
  (bind _buttontop3 (`self.ButtonTop3`))
  (bind _pointlight3 (`self.PointLight3`))
  ;[1 1 1] Button Animations (cant collapse because of timelines)
  (if (== OtherActor (`self.PawnRef`))
    (`/Engine/EditorBlueprintResources/StandardMacros.DoOnce` false :!label _label_5
      (:`Completed`
        (bind (_direction _newtrack_0) (`Timeline|Timeline_0` :!via `PlayFromStart`)
          (:`Update`
            (`SceneComponent.K2_SetRelativeLocation` (`self.BottonPivot3`) (`KismetMathLibrary.VLerp` (0.0 0.0 0.0) (0.231025 0.0 -0.171261) _newtrack_0) false false)
            (if (< _newtrack_0 0.2)
              (`/Engine/EditorBlueprintResources/StandardMacros.DoOnce` false :!label _label_6
                (:`Completed`
                  (`PrimitiveComponent.SetMaterial` _buttontop3 0 "/Game/ProjectCantina/Materials/Console/ButtonMat.ButtonMat")
                  (`SceneComponent.SetVisibility` _pointlight3 true false)
                  (`self.Button3pressed`)))))
          (:`Finished`
            (`|ExecutionSequence`
              (:`then_0`
                (`PrimitiveComponent.SetMaterial` _buttontop3 0 "/Game/ProjectCantina/Materials/Console/HalcyonTextureSheet_Mat.HalcyonTextureSheet_Mat")
                (`SceneComponent.SetVisibility` _pointlight3 false false)
                (`|ExecutionSequence`
                  (:`then_0`
                    (goto _label_5 :!via `Reset`))
                  (:`then_1`
                    (goto _label_6 :!via `Reset`)))))))))))

(event `self.Box4.OnComponentBeginOverlap`
  (params (OverlappedComponent :type "PrimitiveComponent Object Reference") (OtherActor :type "Actor Object Reference") (OtherComp :type "PrimitiveComponent Object Reference") (OtherBodyIndex :type Integer) (bFromSweep :type Boolean) (SweepResult :type "HitResult Structure (by ref)"))
  (bind _buttontop4 (`self.ButtonTop4`))
  (bind _pointlight4 (`self.PointLight4`))
  ;[1 1 1] Button Animations (cant collapse because of timelines)
  (if (== OtherActor (`self.PawnRef`))
    (`/Engine/EditorBlueprintResources/StandardMacros.DoOnce` false :!label _label_7
      (:`Completed`
        (bind (_direction _newtrack_0) (`Timeline|Timeline_1` :!via `PlayFromStart`)
          (:`Update`
            (`SceneComponent.K2_SetRelativeLocation` (`self.BottonPivot4`) (`KismetMathLibrary.VLerp` (0.0 0.0 0.0) (0.231025 0.0 -0.171261) _newtrack_0) false false)
            (if (< _newtrack_0 0.2)
              (`/Engine/EditorBlueprintResources/StandardMacros.DoOnce` false :!label _label_8
                (:`Completed`
                  (`PrimitiveComponent.SetMaterial` _buttontop4 0 "/Game/ProjectCantina/Materials/Console/ButtonMat.ButtonMat")
                  (`SceneComponent.SetVisibility` _pointlight4 true false)
                  (`self.Button4Pressed`)))))
          (:`Finished`
            (`|ExecutionSequence`
              (:`then_0`
                (`PrimitiveComponent.SetMaterial` _buttontop4 0 "/Game/ProjectCantina/Materials/Console/HalcyonTextureSheet_Mat.HalcyonTextureSheet_Mat")
                (`SceneComponent.SetVisibility` _pointlight4 false false)
                (`|ExecutionSequence`
                  (:`then_0`
                    (goto _label_7 :!via `Reset`))
                  (:`then_1`
                    (goto _label_8 :!via `Reset`)))))))))))

(event `self.Box5.OnComponentBeginOverlap`
  (params (OverlappedComponent :type "PrimitiveComponent Object Reference") (OtherActor :type "Actor Object Reference") (OtherComp :type "PrimitiveComponent Object Reference") (OtherBodyIndex :type Integer) (bFromSweep :type Boolean) (SweepResult :type "HitResult Structure (by ref)"))
  (bind _buttontop5 (`self.ButtonTop5`))
  (bind _pointlight5 (`self.PointLight5`))
  ;[1 1 1] Button Animations (cant collapse because of timelines)
  (if (== OtherActor (`self.PawnRef`))
    (`/Engine/EditorBlueprintResources/StandardMacros.DoOnce` false :!label _label_9
      (:`Completed`
        (bind (_direction _newtrack_0) (`Timeline|Timeline_2` :!via `PlayFromStart`)
          (:`Update`
            (`SceneComponent.K2_SetRelativeLocation` (`self.BottonPivot5`) (`KismetMathLibrary.VLerp` (0.0 0.0 0.0) (0.231025 0.0 -0.171261) _newtrack_0) false false)
            (if (< _newtrack_0 0.2)
              (`/Engine/EditorBlueprintResources/StandardMacros.DoOnce` false :!label _label_10
                (:`Completed`
                  (`PrimitiveComponent.SetMaterial` _buttontop5 0 "/Game/ProjectCantina/Materials/Console/ButtonMat.ButtonMat")
                  (`SceneComponent.SetVisibility` _pointlight5 true false)))))
          (:`Finished`
            (`|ExecutionSequence`
              (:`then_0`
                (`PrimitiveComponent.SetMaterial` _buttontop5 0 "/Game/ProjectCantina/Materials/Console/HalcyonTextureSheet_Mat.HalcyonTextureSheet_Mat")
                (`SceneComponent.SetVisibility` _pointlight5 false false)
                (`|ExecutionSequence`
                  (:`then_0`
                    (goto _label_9 :!via `Reset`))
                  (:`then_1`
                    (goto _label_10 :!via `Reset`)))))))))))

(event `self.Box6.OnComponentBeginOverlap`
  (params (OverlappedComponent :type "PrimitiveComponent Object Reference") (OtherActor :type "Actor Object Reference") (OtherComp :type "PrimitiveComponent Object Reference") (OtherBodyIndex :type Integer) (bFromSweep :type Boolean) (SweepResult :type "HitResult Structure (by ref)"))
  (bind _buttontop6 (`self.ButtonTop6`))
  (bind _pointlight6 (`self.PointLight6`))
  ;[1 1 1] Button Animations (cant collapse because of timelines)
  (if (== OtherActor (`self.PawnRef`))
    (`/Engine/EditorBlueprintResources/StandardMacros.DoOnce` false :!label _label_11
      (:`Completed`
        (bind (_direction _newtrack_0) (`Timeline|Timeline_3` :!via `PlayFromStart`)
          (:`Update`
            (`SceneComponent.K2_SetRelativeLocation` (`self.BottonPivot6`) (`KismetMathLibrary.VLerp` (0.0 0.0 0.0) (0.231025 0.0 -0.171261) _newtrack_0) false false)
            (if (< _newtrack_0 0.2)
              (`/Engine/EditorBlueprintResources/StandardMacros.DoOnce` false :!label _label_12
                (:`Completed`
                  (`PrimitiveComponent.SetMaterial` _buttontop6 0 "/Game/ProjectCantina/Materials/Console/ButtonMat.ButtonMat")
                  (`SceneComponent.SetVisibility` _pointlight6 true false)))))
          (:`Finished`
            (`|ExecutionSequence`
              (:`then_0`
                (`PrimitiveComponent.SetMaterial` _buttontop6 0 "/Game/ProjectCantina/Materials/Console/HalcyonTextureSheet_Mat.HalcyonTextureSheet_Mat")
                (`SceneComponent.SetVisibility` _pointlight6 false false)
                (`|ExecutionSequence`
                  (:`then_0`
                    (goto _label_11 :!via `Reset`))
                  (:`then_1`
                    (goto _label_12 :!via `Reset`)))))))))))

(event `self.Box7.OnComponentBeginOverlap`
  (params (OverlappedComponent :type "PrimitiveComponent Object Reference") (OtherActor :type "Actor Object Reference") (OtherComp :type "PrimitiveComponent Object Reference") (OtherBodyIndex :type Integer) (bFromSweep :type Boolean) (SweepResult :type "HitResult Structure (by ref)"))
  (bind _buttontop7 (`self.ButtonTop7`))
  (bind _pointlight7 (`self.PointLight7`))
  ;[1 1 1] Button Animations (cant collapse because of timelines)
  (if (== OtherActor (`self.PawnRef`))
    (`/Engine/EditorBlueprintResources/StandardMacros.DoOnce` false :!label _label_13
      (:`Completed`
        (bind (_direction _newtrack_0) (`Timeline|Timeline_4` :!via `PlayFromStart`)
          (:`Update`
            (`SceneComponent.K2_SetRelativeLocation` (`self.BottonPivot7`) (`KismetMathLibrary.VLerp` (0.0 0.0 0.0) (0.231025 0.0 -0.171261) _newtrack_0) false false)
            (if (< _newtrack_0 0.2)
              (`/Engine/EditorBlueprintResources/StandardMacros.DoOnce` false :!label _label_14
                (:`Completed`
                  (`PrimitiveComponent.SetMaterial` _buttontop7 0 "/Game/ProjectCantina/Materials/Console/ButtonMat.ButtonMat")
                  (`SceneComponent.SetVisibility` _pointlight7 true false)))))
          (:`Finished`
            (`|ExecutionSequence`
              (:`then_0`
                (`PrimitiveComponent.SetMaterial` _buttontop7 0 "/Game/ProjectCantina/Materials/Console/HalcyonTextureSheet_Mat.HalcyonTextureSheet_Mat")
                (`SceneComponent.SetVisibility` _pointlight7 false false)
                (`|ExecutionSequence`
                  (:`then_0`
                    (goto _label_13 :!via `Reset`))
                  (:`then_1`
                    (goto _label_14 :!via `Reset`)))))))))))

(fn `UserConstructionScript`)