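; SequenceSwitcher is a Blueprint that controls which Level Sequence is currently playing.
; PlaySequence stops any active player, then creates and starts a new player for the given sequence, or only stops playback when Play is false.
; SkipIntro applies a hard-coded frame range to the playing sequence, apparently to move past its intro.
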(event `/Game/ProjectCantina/Blueprints/BPI_PawnCommunication.PlaySequence`
  (params (Sequence :type "LevelSequence Object Reference") (` Play?` :type Boolean))
  (bind _sequenceplayer (`self.SequencePlayer`))
  (if ` Play?`
    (`/Engine/EditorBlueprintResources/StandardMacros.IsValid` _sequenceplayer
      (:`Is Valid`
        (if (`MovieSceneSequencePlayer.IsPlaying` _sequenceplayer)
          (`MovieSceneSequencePlayer.Stop` _sequenceplayer)))
      (:`Is Not Valid`
        _))
    (bind (_outactor _returnvalue) (`LevelSequencePlayer.CreateLevelSequencePlayer` Sequence))
    (set `self.SequencePlayer` _returnvalue)
    (`MovieSceneSequencePlayer.Play` _returnvalue)
    (else
      (`/Engine/EditorBlueprintResources/StandardMacros.IsValid` _sequenceplayer
        (:`Is Valid`
          (if (`MovieSceneSequencePlayer.IsPlaying` _sequenceplayer)
            (`MovieSceneSequencePlayer.Stop` _sequenceplayer)))))))

(event `/Game/ProjectCantina/Blueprints/BPI_PawnCommunication.SkipIntro`
  (bind _sequenceplayer (`self.SequencePlayer`))
  (`/Engine/EditorBlueprintResources/StandardMacros.IsValid` _sequenceplayer
    (:`Is Valid`
      (if (`MovieSceneSequencePlayer.IsPlaying` _sequenceplayer)
        (`MovieSceneSequencePlayer.SetFrameRange` _sequenceplayer 837 8200 0.0)))))

(fn `UserConstructionScript`)