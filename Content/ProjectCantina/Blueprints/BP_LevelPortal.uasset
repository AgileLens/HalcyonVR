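; A level portal trigger that moves BP_HalcyonPawn between streamed rooms such as the main hall, lounge, bedroom, cafeteria and climate sim.
; On box overlap it starts a non-blocking load of the sublevel selected by LevelEnum, then calls the pawn's GoToRoomSpawnPoint with TargetInt.
; Only Main Hall portals unload sublevels, namely the ClimateSim and Bedroom scans.
; A timed Locked debounce exists but is disconnected and never runs.
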(event `self.ReceiveBeginPlay`)

(event `self.Box.OnComponentBeginOverlap`
  (params (OverlappedComponent :type "PrimitiveComponent Object Reference") (OtherActor :type "Actor Object Reference") (OtherComp :type "PrimitiveComponent Object Reference") (OtherBodyIndex :type Integer) (bFromSweep :type Boolean) (SweepResult :type "HitResult Structure (by ref)"))
  (bind _asbp_halcyon_pawn (cast `/Game/ProjectCantina/Blueprints/BP_HalcyonPawn` OtherActor))
  (`GameplayStatics.LoadStreamLevelBySoftObjectPtr` (select `/Game/ProjectCantina/Blueprints/Enum_Sublevels` (`self.LevelEnum`) :`NewEnumerator0` "/Game/ProjectCantina/Maps/MainHall.MainHall" :`NewEnumerator1` "/Game/ProjectCantina/Maps/SublightLounge.SublightLounge" :`NewEnumerator2` "/Game/ProjectCantina/Maps/ScannedRooms/BedRoom_Scan.BedRoom_Scan" :`NewEnumerator3` "/Game/ProjectCantina/Maps/ScannedRooms/DiningRoom_Scan.DiningRoom_Scan" :`NewEnumerator4` "/Game/ProjectCantina/Maps/ScannedRooms/ClimateSim_Scan.ClimateSim_Scan" :!type "World Soft Object Reference") true)
  (`/Game/ProjectCantina/Blueprints/BP_HalcyonPawn.GoToRoomSpawnPoint` _asbp_halcyon_pawn (`self.TargetInt`))
  (switch `/Game/ProjectCantina/Blueprints/Enum_Sublevels` (`self.LevelEnum`)
    (:`NewEnumerator0`
      (`GameplayStatics.UnloadStreamLevelBySoftObjectPtr` "/Game/ProjectCantina/Maps/ScannedRooms/ClimateSim_Scan.ClimateSim_Scan")
      (`GameplayStatics.UnloadStreamLevelBySoftObjectPtr` "/Game/ProjectCantina/Maps/ScannedRooms/BedRoom_Scan.BedRoom_Scan"))))

(fn `UserConstructionScript`)