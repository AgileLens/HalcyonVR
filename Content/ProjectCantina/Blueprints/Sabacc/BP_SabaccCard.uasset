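; BP_SabaccCard is a card actor for the Sabacc card game, with a static mesh and two text renders.
; On BeginPlay the mesh uses an overlap-only collision profile for a brief delay, then switches to PhysicsActor and sets its constraint mode to default.
; SetText writes the same card label to both text renders.
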(event `self.ReceiveBeginPlay`
  (bind _staticmesh (`self.StaticMesh`))
  (`PrimitiveComponent.SetCollisionProfileName` _staticmesh "OverlapAllDynamic" true)
  (`KismetSystemLibrary.Delay` 0.2)
  (`PrimitiveComponent.SetCollisionProfileName` _staticmesh "PhysicsActor" true)
  (`PrimitiveComponent.SetConstraintMode` (`self.StaticMesh`) "Default"))

(fn `SetText`
  (params (CardText :type Text))
  (`TextRenderComponent.K2_SetText` (`self.TextRender`) CardText)
  (`TextRenderComponent.K2_SetText` (`self.TextRender1`) CardText))

(fn `UserConstructionScript`)