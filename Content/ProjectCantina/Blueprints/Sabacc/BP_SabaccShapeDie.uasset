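; Sabacc shape die that reports which shape, square, triangle or circle, its current reading shows to a BP_ShapeDieDisplay found in the level.
; A looping timer started on BeginPlay fires a short line trace along its SceneCaptureComponent2D's forward vector.
; The hit component's display name is matched to one of six named face components, setting CurrentValue and updating the display text.
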(event `self.ReceiveBeginPlay`
  (bind _returnvalue (`GameplayStatics.GetActorOfClass` "/Game/ProjectCantina/Blueprints/Sabacc/BP_ShapeDieDisplay.BP_ShapeDieDisplay_C"))
  (set `self.Display` _returnvalue)
  (`KismetSystemLibrary.K2_SetTimerDelegate` (delegate `GetValue`) 0.1 true))

(event `GetValue`
  (bind _scenecapturecomponent2d (`self.SceneCaptureComponent2D`))
  (bind _returnvalue (`SceneComponent.K2_GetComponentLocation` _scenecapturecomponent2d))
  (bind _outhit (`KismetSystemLibrary.LineTraceSingle` :`Start` _returnvalue :`End` (+ _returnvalue (* (`SceneComponent.GetForwardVector` _scenecapturecomponent2d) 50)) :`TraceChannel` "TraceTypeQuery4" :`bIgnoreSelf` false))
  (switch `string` (`KismetSystemLibrary.GetDisplayName` (`.HitComponent` (`GameplayStatics.BreakHitResult` _outhit)))
    (:`BP_SabaccShapeDie.Top_Square`
      (bind _output_get (set `self.CurrentValue` "square" :!label _label)))
    (:`BP_SabaccShapeDie.Bottom_Square`
      (goto _label))
    (:`BP_SabaccShapeDie.Right_Triangle`
      (bind _output_get_2 (set `self.CurrentValue` "triangle" :!label _label_2)))
    (:`BP_SabaccShapeDie.Left_Triangle`
      (goto _label_2))
    (:`BP_SabaccShapeDie.Front_Circle`
      (bind _output_get_3 (set `self.CurrentValue` "circle" :!label _label_3)))
    (:`BP_SabaccShapeDie.Back_Circle`
      (goto _label_3)))
  (`/Game/ProjectCantina/Blueprints/Sabacc/BP_ShapeDieDisplay.UpdateText` (`self.Display`) (`self.CurrentValue`)))

(fn `UserConstructionScript`)