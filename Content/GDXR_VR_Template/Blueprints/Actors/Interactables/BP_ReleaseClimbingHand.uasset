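; VR climbing interactable that tells the player controller to release a climbing hand once it has held on for about three seconds.
; The first-hand grab on C_GrabComponent stores the motion controller and starts a looping timer that accumulates hold time.
; Past the threshold, each tick sends ReleaseClimbingHandMessage with that controller.
; The first-hand drop resets the count and attempts to pause the timer by function name.
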(event `self.C_GrabComponent.FirstHandGrabbed`
  (params (`Motion Controller` :type "MotionControllerComponent Object Reference") (SkeltalMeshHand :type "SkeletalMeshComponent Object Reference") (`Motion Controller Aim` :type "MotionControllerComponent Object Reference"))
  (set `self.Motion Controller` `Motion Controller`)
  (`KismetSystemLibrary.K2_SetTimerDelegate` (delegate `Release Hand After X Time`) 0.02 true))

(event `Release Hand After X Time`
  (bind _output_get (set `self.NewVar` (+ (`self.NewVar`) 0.02)))
  (if (>= _output_get 3.0)
    (message `/Game/GDXR_VR_Template/Blueprints/Interfaces/BPI_Climbing.Release Climbing Hand` (`GameplayStatics.GetPlayerController` 0) (`self.Motion Controller`))))

(event `self.C_GrabComponent.FirstHandDropped`
  (params (`Original Hand Location` :type "Transform Structure") (`Motion Controller` :type "MotionControllerComponent Object Reference") (`Skeletal Mesh Hand` :type "SkeletalMeshComponent Object Reference"))
  (`KismetSystemLibrary.K2_PauseTimer` null "Release Hand After X Time")
  (set `self.NewVar` 0.0))

(fn `UserConstructionScript`)