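; BP_JoyStick is a grabbable VR joystick that drives another actor through its tilt.
; On first-hand grab it snaps the skeletal hand to the stick and starts a looping timer.
; Each tick projects the direction to the motion controller onto the stick's axes, adds pitch and roll, and sends the negated angles to ActorToControl.
; Release calls a pause on that timer by name and zeroes the stick's rotation.
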(event `self.C_GrabComponent.FirstHandGrabbed`
  (params (`Motion Controller` :type "MotionControllerComponent Object Reference") (SkeltalMeshHand :type "SkeletalMeshComponent Object Reference") (`Motion Controller Aim` :type "MotionControllerComponent Object Reference"))
  (`KismetSystemLibrary.PrintString` "GRABBBBED")
  (set `self.Motion Controller` `Motion Controller`)
  (`KismetSystemLibrary.K2_SetTimerDelegate` (delegate `Update Position`) 0.02 true)
  (`/Game/GDXR_VR_Template/Blueprints/C_GrabComponent.Snap Skeletal Hand` (`self.C_GrabComponent`) (`self.Motion Controller`) (`self.SnapHand`) (`self.SnapHand`) SkeltalMeshHand))

(event `Update Position`
  (bind _joy_stick (`self.Joy Stick`))
  (bind _joy_stick_2 (`self.Joy Stick`))
  (bind _joy_stick_3 (`self.Joy Stick`))
  (bind (_relativerotation_roll _relativerotation_pitch) (`KismetMathLibrary.BreakRotator` (`SceneComponent.RelativeRotation` _joy_stick_3)))
  (bind (_returnvalue_roll _returnvalue_pitch) (`KismetMathLibrary.BreakRotator` (`KismetMathLibrary.MakeRotator` (* (`KismetMathLibrary.Dot_VectorVector` (`KismetMathLibrary.Conv_RotatorToVector` (`KismetMathLibrary.FindLookAtRotation` (`SceneComponent.K2_GetComponentLocation` _joy_stick_2) (`SceneComponent.K2_GetComponentLocation` (`self.Motion Controller`)))) (`KismetMathLibrary.GetRightVector` (`SceneComponent.K2_GetComponentRotation` _joy_stick_2))) 10.0) (* (`KismetMathLibrary.Dot_VectorVector` (`KismetMathLibrary.Conv_RotatorToVector` (`KismetMathLibrary.FindLookAtRotation` (`SceneComponent.K2_GetComponentLocation` _joy_stick) (`SceneComponent.K2_GetComponentLocation` (`self.Motion Controller`)))) (* (`KismetMathLibrary.GetForwardVector` (`SceneComponent.K2_GetComponentRotation` _joy_stick)) -1.0)) 10.0))))
  ;[1 1 1] Calculate left Right Position
  (`SceneComponent.K2_AddRelativeRotation` _joy_stick_3 (`KismetMathLibrary.MakeRotator` _returnvalue_roll _returnvalue_pitch) false false)
  (message `/Game/GDXR_VR_Template/Blueprints/Interfaces/BPI_PlayerInteractions.CurrentlyInteracting` (`self.ActorToControl`) 0.0 false (`KismetMathLibrary.MakeVector` (* _relativerotation_roll -1.0) (* _relativerotation_pitch -1.0))))

(event `self.C_GrabComponent.FirstHandDropped`
  (params (`Original Hand Location` :type "Transform Structure") (`Motion Controller` :type "MotionControllerComponent Object Reference") (`Skeletal Mesh Hand` :type "SkeletalMeshComponent Object Reference"))
  (`KismetSystemLibrary.K2_PauseTimer` null "Update Position")
  (`SceneComponent.K2_SetRelativeRotation` :`self` (`self.Joy Stick`)))

(fn `UserConstructionScript`)