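; BP_SlidingButton is an interactable button that slides along a spline's first segment to activate a linked actor.
; On overlap, a looping timer moves the mesh to the overlapping component's closest point on that segment, messaging ActorToActivate as it moves.
; Reaching the end alternately sends activate and deactivate messages, once per press.
; Ending overlap pauses the timer, returns the mesh to the start and re-arms it after a short delay.
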(event `self.StaticMesh.OnComponentBeginOverlap`
  (params (OverlappedComponent :type "PrimitiveComponent Object Reference") (OtherActor :type "Actor Object Reference") (OtherComp :type "PrimitiveComponent Object Reference") (OtherBodyIndex :type Integer) (bFromSweep :type Boolean) (SweepResult :type "HitResult Structure (by ref)"))
  (set `self.Other Comp` OtherComp)
  (`self.SlidingButtonActivate`)
  (bind _returnvalue (`KismetSystemLibrary.K2_SetTimerDelegate` (delegate `Update Button Position`) 0.02 true))
  (set `self.TimerHandle` _returnvalue))

(event `Update Button Position`
  (bind _actor_to_activate (`self.Actor To Activate`))
  (bind _spline (`self.Spline`))
  (bind _returnvalue (`SplineComponent.GetLocationAtSplinePoint` _spline 1 "World"))
  (bind _returnvalue_2 (`KismetMathLibrary.FindClosestPointOnSegment` (`SceneComponent.K2_GetComponentLocation` (`self.Other Comp`)) (`SplineComponent.GetLocationAtSplinePoint` _spline 0 "World") _returnvalue))
  (bind _returnvalue_3 (`KismetMathLibrary.VInterpTo` _returnvalue_2 _returnvalue_2 (`KismetMathLibrary.FClamp` (* (`KismetSystemLibrary.K2_GetTimerElapsedTimeHandle` (`self.TimerHandle`)) 1.5)) 2.0))
  (`SceneComponent.K2_SetWorldLocation` (`self.StaticMesh`) _returnvalue_3 true false)
  (`self.SlidingButtonInProgress`)
  (message `/Game/TemplateContent/Blueprints/Interfaces/BPI_PlayerInteractions.CurrentlyInteracting` (`self.Actor To Activate`) 0.0 false (0.0 0.0 0.0))
  (if (== _returnvalue_3 _returnvalue :`ErrorTolerance` 0.05)
    (`/Engine/EditorBlueprintResources/StandardMacros.DoOnce` false :!label _label
      (:`Completed`
        (`KismetSystemLibrary.K2_PauseTimer` null "Update Button Position")
        (set `self.Other Comp` null)
        (`/Engine/EditorBlueprintResources/StandardMacros.FlipFlop`
          (:`A`
            (message `/Game/TemplateContent/Blueprints/Interfaces/BPI_PlayerInteractions.Activation` _actor_to_activate true))
          (:`B`
            (message `/Game/TemplateContent/Blueprints/Interfaces/BPI_PlayerInteractions.Activation` _actor_to_activate false)))))))

(event `self.StaticMesh.OnComponentEndOverlap`
  (params (OverlappedComponent :type "PrimitiveComponent Object Reference") (OtherActor :type "Actor Object Reference") (OtherComp :type "PrimitiveComponent Object Reference") (OtherBodyIndex :type Integer))
  (set `self.Other Comp` OtherComp)
  (`self.SlidingButtonStop `)
  (`KismetSystemLibrary.K2_PauseTimerHandle` (`self.TimerHandle`))
  (`KismetSystemLibrary.MoveComponentTo` (`self.StaticMesh`) (`SplineComponent.GetLocationAtSplinePoint` (`self.Spline`) 0 "Local"))
  (`KismetSystemLibrary.Delay` 0.2)
  (goto _label :!via `Reset`))

(fn `UserConstructionScript`)