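; BP_FlickSwitch is an interactable switch that toggles between on and off when something begins overlapping its Box.
; Each toggle tilts the Switch component, sends an ActivationMessage to ActorToActivate and calls the FlickSwitchOnOff dispatcher with the new state.
; A DoOnce that resets after a short delay debounces repeated overlaps.
; The construction script applies the OnOff state to both the switch rotation and the target actor.
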(event `self.Box.OnComponentBeginOverlap`
  (params (OverlappedComponent :type "PrimitiveComponent Object Reference") (OtherActor :type "Actor Object Reference") (OtherComp :type "PrimitiveComponent Object Reference") (OtherBodyIndex :type Integer) (bFromSweep :type Boolean) (SweepResult :type "HitResult Structure (by ref)"))
  (bind _actortoactivate (`self.ActorToActivate`))
  (bind _switch (`self.Switch`))
  (`/Engine/EditorBlueprintResources/StandardMacros.DoOnce` false :!label _label
    (:`Completed`
      (if (`self.On/Off`)
        (`SceneComponent.K2_SetRelativeRotation` _switch (`KismetMathLibrary.MakeRotator` 0.0 -40.0) false false)
        (set `self.On/Off` false)
        (message `/Game/TemplateContent/Blueprints/Interfaces/BPI_PlayerInteractions.Activation` _actortoactivate false)
        (`self.FlickSwitchOnOff` false)
        (else
          (`SceneComponent.K2_SetRelativeRotation` _switch (`KismetMathLibrary.MakeRotator` 0.0 40.0) false false)
          (set `self.On/Off` true)
          (message `/Game/TemplateContent/Blueprints/Interfaces/BPI_PlayerInteractions.Activation` _actortoactivate true)
          (`self.FlickSwitchOnOff` true)))
      (`KismetSystemLibrary.Delay` 0.25)
      (goto _label :!via `Reset`))))

(fn `UserConstructionScript`
  (bind _actortoactivate (`self.ActorToActivate`))
  (bind _switch (`self.Switch`))
  (if (`self.On/Off`)
    (`SceneComponent.K2_SetRelativeRotation` _switch (struct :`Pitch` 40.0) false false)
    (message `/Game/TemplateContent/Blueprints/Interfaces/BPI_PlayerInteractions.Activation` _actortoactivate true)
    (else
      (`SceneComponent.K2_SetRelativeRotation` _switch (struct :`Pitch` -40.0) false false)
      (message `/Game/TemplateContent/Blueprints/Interfaces/BPI_PlayerInteractions.Activation` _actortoactivate false))))