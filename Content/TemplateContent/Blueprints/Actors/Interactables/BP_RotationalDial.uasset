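; BP_RotationalDial is an interactable dial meant to be turned by a grabbing motion controller, but its rotation logic is unfinished.
; Grabbing through C_GrabComponent stores the controller's aim and starts a looping timer, which releasing pauses.
; Each timer tick adds a zero local rotation to the static mesh, so the dial stays still.
; An unconnected branch would interpolate RotationValue toward the controller's roll, without feeding the mesh rotation.
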(event `self.C_GrabComponent.FirstHandDropped`
  (params (`Original Hand Location` :type "Transform Structure") (`Motion Controller` :type "MotionControllerComponent Object Reference") (`Skeletal Mesh Hand` :type "SkeletalMeshComponent Object Reference"))
  (`KismetSystemLibrary.K2_PauseTimerHandle` (stale `self.C_GrabComponent.FirstHandGrabbed` _returnvalue)))

(event `self.C_GrabComponent.FirstHandGrabbed`
  (params (`Motion Controller` :type "MotionControllerComponent Object Reference") (SkeltalMeshHand :type "SkeletalMeshComponent Object Reference") (`Motion Controller Aim` :type "MotionControllerComponent Object Reference"))
  (bind _output_get (set `self.Motion Controller Aim` `Motion Controller Aim`))
  (bind _returnvalue (`KismetSystemLibrary.K2_SetTimerDelegate` (delegate `CustomEvent`) 0.02 true)))

(event `CustomEvent`
  (`SceneComponent.K2_AddLocalRotation` (`self.StaticMesh`) (`KismetMathLibrary.MakeRotator` 0.0) false false))

(fn `UserConstructionScript`)