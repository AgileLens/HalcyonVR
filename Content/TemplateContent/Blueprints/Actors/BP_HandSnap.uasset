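; BP_HandSnap is a VR hand snap point that attaches the player's hand mesh to a fixed pose on an object.
; On snap, it passes its Arrow transform and custom blend space to the player controller by message, then fires a hand-attached call.
; When climbable, it enables a cheap box collision on a custom channel and also sends a single-hand climbing message.
; The construction script mirrors the preview mesh for left hands.
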(event `self.ReceiveBeginPlay`
  (bind _box_collision (`self.Box Collision`))
  (if (`self.CanClimb?`)
    ;[1 1 1] We use a box collision so its cheaper to calculate.
    (`PrimitiveComponent.SetCollisionObjectType` _box_collision "ECC_GameTraceChannel4")
    (`PrimitiveComponent.SetCollisionEnabled` _box_collision "QueryAndPhysics")))

(event `/Game/TemplateContent/Blueprints/Interfaces/BPI_HandSnapping.SnapHandPosition`
  (params (`Hand Skeletal Mesh` :type "SkeletalMeshComponent Object Reference") (`Motion Controller` :type "MotionControllerComponent Object Reference") (`Hit Result` :type "HitResult Structure"))
  (bind (_bblockinghit _binitialoverlap _time _distance _location _impactpoint _normal _impactnormal _physmat _hitactor _hitcomponent) (`GameplayStatics.BreakHitResult` `Hit Result`))
  (bind _arrow (`self.Arrow`))
  (message `/Game/TemplateContent/Blueprints/Interfaces/BPI_HandSnapping.AttachHandToObject` (`GameplayStatics.GetPlayerController` 0) (`SceneComponent.K2_GetComponentToWorld` _arrow) `Hand Skeletal Mesh` (`self.Custom Anim Blend Space`) _arrow `Motion Controller` true `Hit Result`)
  (`self.Hand Attached`)
  (if (`self.CanClimb?`)
    (message `/Game/TemplateContent/Blueprints/Interfaces/BPI_Climbing.Single Hand Climbing Position` (`GameplayStatics.GetPlayerController` 0) `Motion Controller` _hitcomponent _hitactor `Hand Skeletal Mesh`)))

(fn `UserConstructionScript`
  (if (`self.IsLeftHand?`)
    (`SceneComponent.SetRelativeScale3D` (`self.StaticMesh`) (-1.0 1.0 1.0))))